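; Seamless linked portal that shows the view through its LinkedPortal and teleports the player between the two.
; Each tick the linked portal's clip-planed scene capture mirrors the player camera into a viewport-sized render target on this portal's material.
; When the camera crosses the portal plane, player transform, control rotation and velocity are mapped to the linked portal.
; Player overlap plays both portals' rock sequences to reveal and enable them; leaving reverses and disables them.
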(event `self.ReceiveBeginPlay`
  (bind (_returnvalue_x _returnvalue_y) (`KismetMathLibrary.BreakVector2D` (`WidgetLayoutLibrary.GetViewportSize`)))
  (`/Engine/EditorBlueprintResources/StandardMacros.IsValid` (`self.Portal_MAT`)
    (:`Is Valid`
      _)
    (:`Is Not Valid`
      (`KismetSystemLibrary.Delay` 0.1)))
  (`self.SetTickGroup` "TG_PostUpdateWork")
  (bind _returnvalue (`KismetMaterialLibrary.CreateDynamicMaterialInstance` "/Game/Developer/BenS/Portal/M_Portal.M_Portal"))
  (bind _output_get (set `self.Portal_MAT` _returnvalue))
  (`PrimitiveComponent.SetMaterial` (`self.Portal`) 0 _output_get)
  (bind _returnvalue_2 (`KismetRenderingLibrary.CreateRenderTarget2D` (`KismetMathLibrary.FTrunc` _returnvalue_x) (`KismetMathLibrary.FTrunc` _returnvalue_y)))
  (bind _output_get_2 (set `self.Portal_RT` _returnvalue_2))
  (`MaterialInstanceDynamic.SetTextureParameterValue` (`self.Portal_MAT`) "Texture" _output_get_2)
  (set `SceneCaptureComponent2D.TextureTarget` (`self.Portal_RT`) (`/Game/Developer/BenS/Portal/BP_SeamlessPortal.PortalCam` (`self.LinkedPortal`)))
  (`self.SetClipPlanes`)
  (`MaterialInstanceDynamic.SetVectorParameterValue` (`self.Portal_MAT`) "OffsetDistance" (`KismetMathLibrary.MakeColor` (.x (* (`SceneComponent.GetForwardVector` (`self.FDirection`)) (`self.OffsetAmount`))) (.y (* (`SceneComponent.GetForwardVector` (`self.FDirection`)) (`self.OffsetAmount`))) (.z (* (`SceneComponent.GetForwardVector` (`self.FDirection`)) (`self.OffsetAmount`)))))
  (`KismetArrayLibrary.Array_Add` (`SceneCaptureComponent.HiddenActors` (`self.PortalCam`)) (`ChildActorComponent.ChildActor` (`self.Rocks`))))

(event `self.ReceiveTick`
  (params (DeltaSeconds :type "Float (single-precision)"))
  (`/Engine/EditorBlueprintResources/StandardMacros.IsValid` (`self.Portal_MAT`)
    (:`Is Valid`
      (`self.UpdateSceneCapture`)
      (`self.CheckViewportSize`)
      (`self.ShouldTeleport`))))

(event `self.PortalRockCollision.OnComponentBeginOverlap`
  (params (OverlappedComponent :type "PrimitiveComponent Object Reference") (OtherActor :type "Actor Object Reference") (OtherComp :type "PrimitiveComponent Object Reference") (OtherBodyIndex :type Integer) (bFromSweep :type Boolean) (SweepResult :type "HitResult Structure (by ref)"))
  (bind _actorsequence (`/Game/Developer/BenS/Portal/BP_Rocks.ActorSequence` (cast `/Game/Developer/BenS/Portal/BP_Rocks` (`ChildActorComponent.ChildActor` (`self.Rocks`)) :!pure true)))
  (bind _actorsequence_2 (`/Game/Developer/BenS/Portal/BP_Rocks.ActorSequence` (cast `/Game/Developer/BenS/Portal/BP_Rocks` (`ChildActorComponent.ChildActor` (`/Game/Developer/BenS/Portal/BP_SeamlessPortal.Rocks` (`self.LinkedPortal`))) :!pure true)))
  (cast `/Game/Developer/BenS/Characters/Blueprints/BP_PlayerTestGuy` OtherActor)
  (`ActorSequenceComponent.PlaySequence` _actorsequence_2)
  (add `MovieSceneSequencePlayer.OnFinished` (`ActorSequenceComponent.SequencePlayer` _actorsequence_2) (delegate `LinkedFinished`))
  (`ActorSequenceComponent.PlaySequence` _actorsequence)
  (add `MovieSceneSequencePlayer.OnFinished` (`ActorSequenceComponent.SequencePlayer` _actorsequence) (delegate `OnFinished`))
  (set `self.IsReversed` false))

(event `LinkedFinished`
  (bind _linkedportal (`self.LinkedPortal`))
  (if (not (`self.IsReversed`))
    (`PrimitiveComponent.SetCollisionProfileName` (`/Game/Developer/BenS/Portal/BP_SeamlessPortal.PlayerDetection` _linkedportal) "OverlapAllDynamic" true)
    (`SceneComponent.SetVisibility` (`/Game/Developer/BenS/Portal/BP_SeamlessPortal.Portal` _linkedportal) true false)))

(event `OnFinished`
  (if (not (`self.IsReversed`))
    (`PrimitiveComponent.SetCollisionProfileName` (`self.PlayerDetection`) "OverlapAllDynamic" true)
    (`SceneComponent.SetVisibility` (`self.Portal`) true false)))

(event `self.PortalRockCollision.OnComponentEndOverlap`
  (params (OverlappedComponent :type "PrimitiveComponent Object Reference") (OtherActor :type "Actor Object Reference") (OtherComp :type "PrimitiveComponent Object Reference") (OtherBodyIndex :type Integer))
  (bind _linkedportal (`self.LinkedPortal`))
  (cast `/Game/Developer/BenS/Characters/Blueprints/BP_PlayerTestGuy` OtherActor)
  (`|ExecutionSequence`
    (:`then_0`
      (`MovieSceneSequencePlayer.PlayReverse` (`ActorSequenceComponent.SequencePlayer` (`/Game/Developer/BenS/Portal/BP_Rocks.ActorSequence` (cast `/Game/Developer/BenS/Portal/BP_Rocks` (`ChildActorComponent.ChildActor` (`/Game/Developer/BenS/Portal/BP_SeamlessPortal.Rocks` (`self.LinkedPortal`))) :!pure true))))
      (`MovieSceneSequencePlayer.PlayReverse` (`ActorSequenceComponent.SequencePlayer` (`/Game/Developer/BenS/Portal/BP_Rocks.ActorSequence` (cast `/Game/Developer/BenS/Portal/BP_Rocks` (`ChildActorComponent.ChildActor` (`self.Rocks`)) :!pure true))))
      (set `self.IsReversed` true))
    (:`then_1`
      (if (`self.IsReversed`)
        (`PrimitiveComponent.SetCollisionProfileName` (`/Game/Developer/BenS/Portal/BP_SeamlessPortal.PlayerDetection` _linkedportal) "NoCollision" true)
        (`SceneComponent.SetVisibility` (`/Game/Developer/BenS/Portal/BP_SeamlessPortal.Portal` _linkedportal) false false)
        (`PrimitiveComponent.SetCollisionProfileName` (`self.PlayerDetection`) "NoCollision" true)
        (`SceneComponent.SetVisibility` (`self.Portal`) false false)))))

(fn `CheckViewportSize`
  (bind _portal_rt (`self.Portal_RT`))
  (bind (_x _y) (`KismetMathLibrary.BreakVector2D` (`WidgetLayoutLibrary.GetViewportSize`)))
  (bind (_x_2 _y_2) (`KismetMathLibrary.BreakVector2D` (`WidgetLayoutLibrary.GetViewportSize`)))
  (if (not (and (== _x (`TextureRenderTarget2D.SizeX` _portal_rt)) (== _y (`TextureRenderTarget2D.SizeY` _portal_rt))))
    (`KismetRenderingLibrary.ResizeRenderTarget2D` (`self.Portal_RT`) (`KismetMathLibrary.FTrunc` _x_2) (`KismetMathLibrary.FTrunc` _y_2))))

(fn `IsPointCrossingPortal`
  (params (Point :type "Vector Structure") (`Portal Location` :type "Vector Structure") (PortalNormal :type "Vector Structure"))
  (returns (Return :type Boolean))
  (locals (IsInFront :type Boolean) (PortalPlane :type "Plane Structure") (IsIntersect :type Boolean :default false) (IsCrossing :type Boolean :default false))
  (set `local.IsInFront` (>= (`KismetMathLibrary.Dot_VectorVector` PortalNormal (- Point `Portal Location`)) 0.0))
  (bind _output_get (set `local.PortalPlane` (`KismetMathLibrary.MakePlaneFromPointAndNormal` (`local.Portal Location`) (`local.PortalNormal`))))
  (set `local.IsIntersect` (`.ReturnValue` (`KismetMathLibrary.LinePlaneIntersection` (`self.LastPosition`) (`local.Point`) _output_get)))
  (set `local.IsCrossing` (and (`local.IsIntersect`) (not (`local.IsInFront`)) (`self.LastInFront`)))
  (set `self.LastInFront` (`local.IsInFront`))
  (set `self.LastPosition` (`local.Point`))
  (return (`local.IsCrossing`)))

(fn `SetClipPlanes`
  (bind _portalcam (`self.PortalCam`))
  (`/Engine/EditorBlueprintResources/StandardMacros.IsValid` (`self.LinkedPortal`)
    (:`Is Valid`
      (set `SceneCaptureComponent2D.bEnableClipPlane` true _portalcam)
      (set `SceneCaptureComponent2D.ClipPlaneBase` (+ (`SceneComponent.K2_GetComponentLocation` (`self.Portal`)) (* (`SceneComponent.GetForwardVector` (`self.FDirection`)) 3.0)) _portalcam)
      (set `SceneCaptureComponent2D.ClipPlaneNormal` (`SceneComponent.GetForwardVector` (`self.FDirection`)) _portalcam))))

(fn `ShouldTeleport`
  (`/Engine/EditorBlueprintResources/StandardMacros.IsValid` (`|GetArrayItem` (`PrimitiveComponent.GetOverlappingActors` (`self.PlayerDetection`) "/Game/Developer/BenS/Characters/Blueprints/BP_PlayerTestGuy.BP_PlayerTestGuy_C"))
    (:`Is Valid`
      (bind _return (`self.IsPointCrossingPortal` (`SceneComponent.K2_GetComponentLocation` (`PlayerCharacter.m_Camera` (cast `/Game/Developer/BenS/Characters/Blueprints/BP_PlayerTestGuy` (`GameplayStatics.GetPlayerCharacter` 0) :!pure true))) (`self.K2_GetActorLocation`) (`SceneComponent.GetForwardVector` (`self.FDirection`))))
      (if _return
        (`self.Teleport`)))))

(fn `Teleport`
  (bind _returnvalue (`self.GetTransform`))
  (bind (_returnvalue_location _returnvalue_rotation _returnvalue_scale) (`KismetMathLibrary.BreakTransform` (`self.GetTransform`)))
  (bind _returnvalue_2 (`self.GetTransform`))
  (bind _returnvalue_3 (`Pawn.GetMovementComponent` (`GameplayStatics.GetPlayerCharacter` 0)))
  (bind (_x _y _z) (`KismetMathLibrary.GetAxes` (`Pawn.GetControlRotation` (`GameplayStatics.GetPlayerCharacter` 0))))
  (bind (_x_2 _y_2 _z_2) (`KismetMathLibrary.GetAxes` (`self.K2_GetActorRotation` (`GameplayStatics.GetPlayerCharacter` 0))))
  (`self.K2_SetActorTransform` (`GameplayStatics.GetPlayerCharacter` 0) (`KismetMathLibrary.MakeTransform` (`KismetMathLibrary.TransformLocation` (`self.GetTransform` (`self.LinkedPortal`)) (`KismetMathLibrary.InverseTransformLocation` (`KismetMathLibrary.MakeTransform` _returnvalue_location _returnvalue_rotation (`KismetMathLibrary.MakeVector` (* (.x _returnvalue_scale) -1.0) (* (.y _returnvalue_scale) -1.0) (.z _returnvalue_scale))) (`self.K2_GetActorLocation` (`GameplayStatics.GetPlayerCharacter` 0)))) (`KismetMathLibrary.MakeRotationFromAxes` (`KismetMathLibrary.TransformDirection` (`self.GetTransform` (`self.LinkedPortal`)) (`KismetMathLibrary.MirrorVectorByNormal` (`KismetMathLibrary.MirrorVectorByNormal` (`KismetMathLibrary.InverseTransformDirection` _returnvalue_2 _x_2) (1.0 0.0 0.0)) (0.0 1.0 0.0))) (`KismetMathLibrary.TransformDirection` (`self.GetTransform` (`self.LinkedPortal`)) (`KismetMathLibrary.MirrorVectorByNormal` (`KismetMathLibrary.MirrorVectorByNormal` (`KismetMathLibrary.InverseTransformDirection` _returnvalue_2 _y_2) (1.0 0.0 0.0)) (0.0 1.0 0.0))) (`KismetMathLibrary.TransformDirection` (`self.GetTransform` (`self.LinkedPortal`)) (`KismetMathLibrary.MirrorVectorByNormal` (`KismetMathLibrary.MirrorVectorByNormal` (`KismetMathLibrary.InverseTransformDirection` _returnvalue_2 _z_2) (1.0 0.0 0.0)) (0.0 1.0 0.0))))) false false)
  (`Controller.SetControlRotation` (`GameplayStatics.GetPlayerController` 0) (`KismetMathLibrary.MakeRotationFromAxes` (`KismetMathLibrary.TransformDirection` (`self.GetTransform` (`self.LinkedPortal`)) (`KismetMathLibrary.MirrorVectorByNormal` (`KismetMathLibrary.MirrorVectorByNormal` (`KismetMathLibrary.InverseTransformDirection` _returnvalue _x) (1.0 0.0 0.0)) (0.0 1.0 0.0))) (`KismetMathLibrary.TransformDirection` (`self.GetTransform` (`self.LinkedPortal`)) (`KismetMathLibrary.MirrorVectorByNormal` (`KismetMathLibrary.MirrorVectorByNormal` (`KismetMathLibrary.InverseTransformDirection` _returnvalue _y) (1.0 0.0 0.0)) (0.0 1.0 0.0))) (`KismetMathLibrary.TransformDirection` (`self.GetTransform` (`self.LinkedPortal`)) (`KismetMathLibrary.MirrorVectorByNormal` (`KismetMathLibrary.MirrorVectorByNormal` (`KismetMathLibrary.InverseTransformDirection` _returnvalue _z) (1.0 0.0 0.0)) (0.0 1.0 0.0)))))
  (bind _returnvalue_4 (`self.UpdateVelocity` (`MovementComponent.Velocity` _returnvalue_3)))
  (set `MovementComponent.Velocity` _returnvalue_4 _returnvalue_3))

(fn `UpdateLocation`
  (params (OldLocation :type "Vector Structure"))
  (returns (ReturnValue :type "Vector Structure"))
  ; Update Location
  (return (`KismetMathLibrary.TransformLocation` (`self.GetTransform` (`self.LinkedPortal`)) (`KismetMathLibrary.InverseTransformLocation` (`KismetMathLibrary.MakeTransform` (.location (`self.GetTransform`)) (.rotation (`self.GetTransform`)) (`KismetMathLibrary.MakeVector` (* (.x (.scale (`self.GetTransform`))) -1.0) (* (.y (.scale (`self.GetTransform`))) -1.0) (.z (.scale (`self.GetTransform`))))) OldLocation))))

(fn `UpdateRotation`
  (params (OldRotation :type "Rotator Structure"))
  (returns (ReturnValue :type "Rotator Structure"))
  (bind (_x _y _z) (`KismetMathLibrary.BreakRotIntoAxes` OldRotation))
  (bind _returnvalue (`self.GetTransform`))
  (bind _returnvalue_2 (`self.GetTransform` (`self.LinkedPortal`)))
  ; UpdateRotation
  (return (`KismetMathLibrary.MakeRotationFromAxes` (`KismetMathLibrary.TransformDirection` _returnvalue_2 (`KismetMathLibrary.MirrorVectorByNormal` (`KismetMathLibrary.MirrorVectorByNormal` (`KismetMathLibrary.InverseTransformDirection` _returnvalue _x) (1.0 0.0 0.0)) (0.0 1.0 0.0))) (`KismetMathLibrary.TransformDirection` _returnvalue_2 (`KismetMathLibrary.MirrorVectorByNormal` (`KismetMathLibrary.MirrorVectorByNormal` (`KismetMathLibrary.InverseTransformDirection` _returnvalue _y) (1.0 0.0 0.0)) (0.0 1.0 0.0))) (`KismetMathLibrary.TransformDirection` _returnvalue_2 (`KismetMathLibrary.MirrorVectorByNormal` (`KismetMathLibrary.MirrorVectorByNormal` (`KismetMathLibrary.InverseTransformDirection` _returnvalue _z) (1.0 0.0 0.0)) (0.0 1.0 0.0))))))

(fn `UpdateSceneCapture`
  (`SceneComponent.K2_SetWorldLocationAndRotation` (`/Game/Developer/BenS/Portal/BP_SeamlessPortal.PortalCam` (`self.LinkedPortal`)) (`self.UpdateLocation` (`SceneComponent.K2_GetComponentLocation` (`PlayerCameraManager.TransformComponent` (`GameplayStatics.GetPlayerCameraManager` 0)))) (`self.UpdateRotation` (`SceneComponent.K2_GetComponentRotation` (`PlayerCameraManager.TransformComponent` (`GameplayStatics.GetPlayerCameraManager` 0)))) false false))

(fn `UpdateVelocity`
  (params (Velocity :type "Vector Structure"))
  (returns (ReturnValue :type "Vector Structure"))
  (return (* (`KismetMathLibrary.TransformDirection` (`self.GetTransform` (`self.LinkedPortal`)) (`KismetMathLibrary.MirrorVectorByNormal` (`KismetMathLibrary.MirrorVectorByNormal` (`KismetMathLibrary.InverseTransformDirection` (`self.GetTransform`) (`KismetMathLibrary.Normal` Velocity)) (1.0 0.0 0.0)) (0.0 1.0 0.0))) (`KismetMathLibrary.VSize` (`local.Velocity`)))))

(fn `UserConstructionScript`)