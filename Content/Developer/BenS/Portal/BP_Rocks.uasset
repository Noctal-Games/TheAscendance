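; BP_Rocks is a rock Blueprint in a developer Portal folder, built from nineteen static mesh components.
; Its construction script gathers those components into the RockSelection array in a hand-set, non-numeric order.
; It has no other graph logic, and nothing here reads the array.
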(fn `UserConstructionScript`
  (set `self.RockSelection` (`|MakeArray` (`self.StaticMesh7`) (`self.StaticMesh2`) (`self.StaticMesh3`) (`self.StaticMesh4`) (`self.StaticMesh5`) (`self.StaticMesh6`) (`self.StaticMesh9`) (`self.StaticMesh15`) (`self.StaticMesh16`) (`self.StaticMesh1`) (`self.StaticMesh17`) (`self.StaticMesh18`) (`self.StaticMesh14`) (`self.StaticMesh8`) (`self.StaticMesh`) (`self.StaticMesh10`) (`self.StaticMesh11`) (`self.StaticMesh12`) (`self.StaticMesh13`))))