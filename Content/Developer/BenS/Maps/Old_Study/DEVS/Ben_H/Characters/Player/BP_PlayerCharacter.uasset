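; Player character Blueprint with two-handed combo attacks, a timeline dodge along a sphere trace, and a separate hand mesh with a spell cast socket.
; Attack montages advance a shared combo index that resets after a delay.
; Gait settings drive movement and animation, while a per-tick ground trace feeds distance matching.
; It also handles arm-bone visibility, hit feedback, death and recovery, a loadout widget, and interface-based proximity and dialogue interaction.
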(event `EnhancedInput|/Game/Developer/BenS/Maps/Old_Study/DEVS/Ben_H/Input/IA_MainHandPrimaryAttack`
  (params (ActionValue :type Boolean) (ElapsedSeconds :type "Float (double-precision)") (TriggeredSeconds :type "Float (double-precision)") (InputAction :type "InputAction Object Reference" :default "/Game/Developer/BenS/Maps/Old_Study/DEVS/Ben_H/Input/IA_MainHandPrimaryAttack.IA_MainHandPrimaryAttack"))
  ;[0.07292 0.07292 0.07292] Combo System
  (:`Triggered`
    (bind _returnvalue (`self.IsMainHandAttacking`))
    (if _returnvalue
      (if (`self.CanCombo`)
        (bind _animation (`self.MainHandCombo`))
        (`|PlayMontage` (`self.SkeletalMesh`) _animation
          (:`then`
            (set `self.CanCombo` false)))))))

(event `EnhancedInput|/Game/Developer/BenS/Maps/Old_Study/DEVS/Ben_H/Input/IA_OffhandPrimaryAttack`
  (params (ActionValue :type Boolean) (ElapsedSeconds :type "Float (double-precision)") (TriggeredSeconds :type "Float (double-precision)") (InputAction :type "InputAction Object Reference" :default "/Game/Developer/BenS/Maps/Old_Study/DEVS/Ben_H/Input/IA_OffhandPrimaryAttack.IA_OffhandPrimaryAttack"))
  ;[0.07292 0.07292 0.07292] Combo System
  (:`Triggered`
    (bind _returnvalue (`self.IsOffhandAttacking`))
    (if _returnvalue
      (if (`self.CanCombo`)
        (bind _animation (`self.OffhandCombo`))
        (`|PlayMontage` (`self.SkeletalMesh`) _animation
          (:`then`
            (set `self.CanCombo` false)))))))

(event `EnhancedInput|/Game/Developer/BenS/Maps/Old_Study/DEVS/Ben_H/Input/IA_MainHandAltAttack`
  (params (ActionValue :type Boolean) (ElapsedSeconds :type "Float (double-precision)") (TriggeredSeconds :type "Float (double-precision)") (InputAction :type "InputAction Object Reference" :default "/Game/Developer/BenS/Maps/Old_Study/DEVS/Ben_H/Input/IA_MainHandAltAttack.IA_MainHandAltAttack"))
  ;[0.07292 0.07292 0.07292] Combo System
  (:`Triggered`
    (bind _returnvalue (`self.IsMainHandAttacking`))
    (if _returnvalue
      (`|PlayMontage` (`self.SkeletalMesh`)))))

(event `ContinueCombo`
  ;[0.07292 0.07292 0.07292] Combo System
  (`/Engine/EditorBlueprintResources/StandardMacros.IncrementInt` (`self.ComboIndex`)
    (:`  `
      (`KismetSystemLibrary.RetriggerableDelay` 1.0)
      (set `self.ComboIndex` 0 :!label _label))))

(event `EnhancedInput|/Game/Developer/BenS/Maps/Old_Study/DEVS/Ben_H/Input/IA_Ready`
  (params (ActionValue :type Boolean) (ElapsedSeconds :type "Float (double-precision)") (TriggeredSeconds :type "Float (double-precision)") (InputAction :type "InputAction Object Reference" :default "/Game/Developer/BenS/Maps/Old_Study/DEVS/Ben_H/Input/IA_Ready.IA_Ready")))

(event `ResetCombo`
  ;[0.07292 0.07292 0.07292] Combo System
  (goto _label))

(event `ResetIsReady`
  (`/Engine/EditorBlueprintResources/StandardMacros.DoOnce` false :!via `Reset`
    (:`Completed`
      (`/Engine/EditorBlueprintResources/StandardMacros.FlipFlop`
        (:`A`
          (set `self.IsReady` true)
          (for _array_element (`self.Arms`)
            (`SkinnedMeshComponent.HideBoneByName` (`self.Mesh`) _array_element "PBO_None")
            (`KismetSystemLibrary.Delay` 0.8)
            (`self.ResetIsReady`)))
        (:`B`
          (set `self.IsReady` false)
          (`KismetSystemLibrary.Delay` 0.8)
          (for _array_element_2 (`self.Arms`)
            (`SkinnedMeshComponent.UnHideBoneByName` (`self.Mesh`) _array_element_2)
            (`self.ResetIsReady`)))))))

(event `EnhancedInput|/Game/Developer/BenS/Maps/Old_Study/DEVS/Ben_H/Input/IA_OffhandAltAttack`
  (params (ActionValue :type Boolean) (ElapsedSeconds :type "Float (double-precision)") (TriggeredSeconds :type "Float (double-precision)") (InputAction :type "InputAction Object Reference" :default "/Game/Developer/BenS/Maps/Old_Study/DEVS/Ben_H/Input/IA_OffhandAltAttack.IA_OffhandAltAttack"))
  ;[0.07292 0.07292 0.07292] Combo System
  (:`Triggered`
    (bind _returnvalue (`self.IsOffhandAttacking`))
    (if _returnvalue
      (`|PlayMontage` (`self.SkeletalMesh`)))))

(event `EnhancedInput|/Game/Developer/BenS/Maps/Old_Study/DEVS/Ben_H/Input/IA_Dodge`
  (params (ActionValue :type Boolean) (ElapsedSeconds :type "Float (double-precision)") (TriggeredSeconds :type "Float (double-precision)") (InputAction :type "InputAction Object Reference" :default "/Game/Developer/BenS/Maps/Old_Study/DEVS/Ben_H/Input/IA_Dodge.IA_Dodge"))
  (bind _returnvalue (`self.K2_GetActorLocation`))
  (:`Triggered`
    (`/Engine/EditorBlueprintResources/StandardMacros.DoOnce` false :!label _label_2
      (:`Completed`
        (set `self.IsDodging` true)
        (bind _outhit (`KismetSystemLibrary.SphereTraceSingle` _returnvalue (+ _returnvalue (* (`KismetMathLibrary.Normal` (`self.GetLastMovementInputVector`)) (`self.Dodge Distance`))) 10.0 "TraceTypeQuery1"))
        (bind (_direction _dodge) (`Timeline|Timeline` :!via `PlayFromStart`)
          (:`Update`
            (bind (_bblockinghit _binitialoverlap _time _distance _location _impactpoint _normal _impactnormal _physmat _hitactor _hitcomponent _hitbonename _bonename _hititem _elementindex _faceindex _tracestart _traceend) (`GameplayStatics.BreakHitResult` _outhit))
            (`self.K2_SetActorLocation` (`KismetMathLibrary.VLerp` _tracestart _traceend _dodge) true)
            (`KismetSystemLibrary.Delay` (`self.DodgeCoolDown`))
            (goto _label_2 :!via `Reset`))
          (:`Finished`
            (set `self.IsDodging` false)))))))

(event `self.ReceiveTick`
  (params (DeltaSeconds :type "Float (single-precision)"))
  (`self.DistanceMatching`))

(event `self.ReceiveBeginPlay`
  (`|ExecutionSequence`
    (:`then_0`
      (`self.SetHandMesh` (`self.SkeletalMesh`))
      (`self.BindSpellVFXToSocket` (`self.SkeletalMesh`) "CastPoint")
      (bind _asplayer_movement_component (cast `` (`self.CharacterMovement`)))
      (set `self.PlayerMovement` _asplayer_movement_component)
      (`self.UpdateGait` 0)
      (`SkeletalMeshComponent.LinkAnimClassLayers` (`self.Mesh`) null)
      (message `/Game/Developer/BenS/Maps/Old_Study/DEVS/Ben_H/Characters/Player/BP_PlayerCharacter.ReceiveOverlayState` (`SkeletalMeshComponent.GetAnimInstance` (`self.Mesh`)) 0)
      (add `self.OnDeath` (delegate `OnDeath_Event`))
      (add `self.OnHit` (delegate `OnHitEvent`))
      (add `self.OnTakeDamage` (delegate `OnTakeDamageEvent`)))
    (:`then_1`
      (for _array_element (`self.Arms`)
        (`SkinnedMeshComponent.HideBoneByName` (`self.Mesh`) _array_element "PBO_None")
        (`SkinnedMeshComponent.HideBoneByName` (`self.SkeletalMesh`) (`self.HeadBone`) "PBO_None")))))

(event `OnDeath_Event` :!signature `self.OnDeath`
  (params (character :type "Object Object Reference"))
  (bind _mesh (`Character.Mesh` character))
  (set `self.HasDied` true)
  (`GameplayStatics.PlaySound2D` null 1.0 1.0 0.0 null null)
  (set `self.IsReady` false)
  (`|ExecutionSequence`
    (:`then_0`
      (for _array_element (`self.Arms`)
        (`SkinnedMeshComponent.UnHideBoneByName` _mesh _array_element)))
    (:`then_1`
      (`SkeletalMeshComponent.PlayAnimation` _mesh null false)
      (`self.DisableInput` (`GameplayStatics.GetPlayerController` 0))
      (`KismetSystemLibrary.Delay` 0.7)
      (`SkeletalMeshComponent.UnlinkAnimClassLayers` _mesh null)
      (bind _returnvalue (`|CreateWidget` null))
      (`UserWidget.AddToViewport` _returnvalue 0)
      (`self.UpdateGait` 0)
      (`SkeletalMeshComponent.SetAnimInstanceClass` _mesh null)
      (`SkeletalMeshComponent.LinkAnimClassLayers` _mesh null)
      (message `/Game/Developer/BenS/Maps/Old_Study/DEVS/Ben_H/Characters/Player/BP_PlayerCharacter.ReceiveOverlayState` (`SkeletalMeshComponent.GetAnimInstance` _mesh) 0)
      (`self.EnableInput` (`GameplayStatics.GetPlayerController` 0))
      (set `self.HasDied` false))))

(event `OnHitEvent`
  (bind _returnvalue (`|CreateWidget` null))
  (`UserWidget.AddToViewport` _returnvalue 0)
  (`GameplayStatics.PlayWorldCameraShake` null (`SceneComponent.K2_GetComponentLocation` (`self.Mesh`)) 0.0 500.0)
  (`GameplayStatics.PlaySound2D` null 1.0 1.0 0.0 null null))

(event `EnhancedInput|/Game/Developer/BenS/Maps/Old_Study/DEVS/Ben_H/Input/IA_TogglePause`
  (params (ActionValue :type Boolean) (ElapsedSeconds :type "Float (double-precision)") (TriggeredSeconds :type "Float (double-precision)") (InputAction :type "InputAction Object Reference" :default "/Game/Developer/BenS/Maps/Old_Study/DEVS/Ben_H/Input/IA_TogglePause.IA_TogglePause"))
  (bind _returnvalue (subsystem ``))
  (:`Triggered`
    (`/Engine/EditorBlueprintResources/StandardMacros.IsValid` _returnvalue
      (:`Is Valid`
        (`self.Contains` _returnvalue 0)))))

(event `OnTakeDamageEvent`
  (`GameplayStatics.PlaySound2D` null 1.0 1.0 0.0 null null)
  (bind _returnvalue (`|CreateWidget` null))
  (`UserWidget.AddToViewport` _returnvalue 0))

(event `Key|O`
  (params (Key :type "Key Structure"))
  (bind _returnvalue (`GameplayStatics.GetPlayerController` 0))
  (:`Pressed`
    (`/Engine/EditorBlueprintResources/StandardMacros.FlipFlop`
      (:`A`
        (`WidgetBlueprintLibrary.SetInputMode_GameAndUIEx` _returnvalue null "DoNotLock" false)
        (set `PlayerController.bShowMouseCursor` true _returnvalue)
        (bind _returnvalue_2 (`|CreateWidget` null))
        (bind _output_get (set `self.LoadoutWidget` _returnvalue_2))
        (`UserWidget.AddToViewport` _output_get 0))
      (:`B`
        (`WidgetBlueprintLibrary.SetInputMode_GameOnly` _returnvalue)
        (set `PlayerController.bShowMouseCursor` false _returnvalue)
        (`Widget.RemoveFromParent` (`self.LoadoutWidget`))))))

(event `self._proximitySensor.OnComponentBeginOverlap`
  (params (OverlappedComponent :type "PrimitiveComponent Object Reference") (OtherActor :type "Actor Object Reference") (OtherComp :type "PrimitiveComponent Object Reference") (OtherBodyIndex :type Integer) (bFromSweep :type Boolean) (SweepResult :type "HitResult Structure (by ref)"))
  (if (`KismetSystemLibrary.DoesImplementInterface` OtherActor)
    (message `/Game/Developer/BenS/Maps/Old_Study/DEVS/Ben_H/Characters/Player/BP_PlayerCharacter.InRange` OtherActor self)))

(event `self._proximitySensor.OnComponentEndOverlap`
  (params (OverlappedComponent :type "PrimitiveComponent Object Reference") (OtherActor :type "Actor Object Reference") (OtherComp :type "PrimitiveComponent Object Reference") (OtherBodyIndex :type Integer))
  (if (`KismetSystemLibrary.DoesImplementInterface` OtherActor)
    (message `/Game/Developer/BenS/Maps/Old_Study/DEVS/Ben_H/Characters/Player/BP_PlayerCharacter.InRangeExited` OtherActor self)))

(event `Key|E`
  (params (Key :type "Key Structure"))
  (:`Pressed`
    (for _array_element (`self.GetOverlappingActors` null)
      (if (`KismetSystemLibrary.DoesImplementInterface` _array_element "/Game/Developer/BenS/Maps/Old_Study/DEVS/Ben_K/Dialogue/BPI_Dialogue.BPI_Dialogue_C")
        (message `/Game/Developer/BenS/Maps/Old_Study/DEVS/Ben_K/Dialogue/BPI_Dialogue.Talk` _array_element)))))

(fn `DistanceMatching`
  (bind _returnvalue (`self.K2_GetActorLocation`))
  (bind (_outhit _returnvalue_2) (`KismetSystemLibrary.SphereTraceSingle` (- _returnvalue (`KismetMathLibrary.MakeVector` 0.0 0.0 (`CapsuleComponent.CapsuleHalfHeight` (`self.CapsuleComponent`)))) (- _returnvalue (0.0 0.0 -1000.0)) (`CapsuleComponent.CapsuleRadius` (`self.CapsuleComponent`)) "TraceTypeQuery1"))
  (if _returnvalue_2
    (message `/Game/Developer/BenS/Maps/Old_Study/DEVS/Ben_H/Characters/Player/BP_PlayerCharacter.ReceiveGroundDistance` (`SkeletalMeshComponent.GetAnimInstance` (`self.Mesh`)) (`.Distance` (`GameplayStatics.BreakHitResult` _outhit)))))

(fn `GetCastStartLocation`
  (returns (ReturnValue :type "Vector Structure"))
  (return (`SceneComponent.GetSocketLocation` (`self.SkeletalMesh`) "CastPoint")))

(fn `MainHandCombo`
  (returns (animation :type "AnimMontage Object Reference"))
  (bind _mainhandattacks (`self.MainHandAttacks`))
  (if (>= (`self.ComboIndex`) (- (`KismetArrayLibrary.Array_Length` (`self.MainHandAttacks`)) 1))
    (`self.ResetCombo`)
    (return (`|GetArrayItem` _mainhandattacks (`KismetArrayLibrary.Array_LastIndex` _mainhandattacks)))
    (else
      (`self.ContinueCombo`)
      (return (`|GetArrayItem` (`self.MainHandAttacks`) (- (`self.ComboIndex`) 1))))))

(fn `OffhandCombo`
  (returns (animation :type "AnimMontage Object Reference"))
  (bind _offhandattacks (`self.OffhandAttacks`))
  (if (>= (`self.ComboIndex`) (- (`KismetArrayLibrary.Array_Length` (`self.OffhandAttacks`)) 1))
    (`self.ResetCombo`)
    (return (`|GetArrayItem` _offhandattacks (`KismetArrayLibrary.Array_LastIndex` _offhandattacks)))
    (else
      (`self.ContinueCombo`)
      (return (`|GetArrayItem` (`self.OffhandAttacks`) (- (`self.ComboIndex`) 1))))))

(fn `UpdateGait`
  (params (DesiredGait :type Byte :default 0))
  (bind _playermovement (`self.PlayerMovement`))
  (bind (_maxacceleration _brakingacceleration _brakingfrictionfactor _buseseparatebrakingfriction _brakingfriction) (break `` (`BlueprintMapLibrary.Map_Find` :`Key` (`local.DesiredGait`))))
  (set `self.f_PreviousGait` (`self.f_currentGait`))
  (set `self.f_currentGait` DesiredGait)
  (message `/Game/Developer/BenS/Maps/Old_Study/DEVS/Ben_H/Characters/Player/BP_PlayerCharacter.ReceiveGaitData` (`SkeletalMeshComponent.GetAnimInstance` (`self.Mesh`)) (`local.DesiredGait`))
  (set `CharacterMovementComponent.MaxAcceleration` _maxacceleration _playermovement)
  (set `CharacterMovementComponent.BrakingDecelerationWalking` _brakingacceleration _playermovement)
  (set `CharacterMovementComponent.BrakingFrictionFactor` _brakingfrictionfactor _playermovement)
  (set `CharacterMovementComponent.bUseSeparateBrakingFriction` _buseseparatebrakingfriction _playermovement)
  (set `CharacterMovementComponent.BrakingFriction` _brakingfriction _playermovement))

(fn `UserConstructionScript`)