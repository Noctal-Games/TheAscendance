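; Grimoire interactable actor that unlocks a set of spells, listed by ID, through a subsystem.
; BeginPlay binds the interact event; UnlockSpells passes each ID to the subsystem and unbinds that event, and still carries a debug print.
; Entering range creates a screen-space prompt widget at UILocation, and leaving reverses its Appear animation, then destroys the component after a short delay.
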(event `self.ReceiveBeginPlay`
  (add `self.OnInteract` (`|CreateDelegate` :!event `Unlock Spells`)))

(event `self.InRange`
  (params (Player :type "Object Object Reference"))
  (`self.InteractionWidgetComponent`
    (:`then`)
    (:`else`
      (bind _returnvalue (`|CreateWidget` null null (`self.InteractIcon`) (`self.InteractText`)))
      (bind _output_get (set `self.Interact` _returnvalue))
      (bind _returnvalue_2 (`AddComponent|NODE_AddWidgetComponent-0`))
      (bind _output_get_2 (set `self.InteractionWidgetComponent` _returnvalue_2))
      (`WidgetComponent.SetWidget` _output_get_2 _output_get)
      (`WidgetComponent.SetWidgetSpace` _output_get_2 "Screen")
      (`WidgetComponent.SetDrawAtDesiredSize` _output_get_2 true)
      (`PrimitiveComponent.SetCollisionEnabled` _output_get_2 "NoCollision")
      (`SceneComponent.K2_AttachToComponent` _output_get_2 (`self.UI_Location`) "None" "SnapToTarget" "SnapToTarget" "SnapToTarget" true))))

(event `self.InRangeExited`
  (params (Player :type "Object Object Reference"))
  (bind _interact (`self.Interact`))
  (bind _interactionwidgetcomponent (`self.InteractionWidgetComponent`)
    (:`then`
      (`UserWidget.PlayAnimation` _interact (`/Game/Developer/BenS/Maps/Old_Study/DEVS/Ben_H/Blueprints/Actors/BP_SpellUnlockGrimoireActor.appear` _interact) 0.0 1 "Reverse" 1.0 false)
      (`KismetSystemLibrary.Delay` 0.2)
      (`ActorComponent.K2_DestroyComponent` _interactionwidgetcomponent))
    (:`else`)))

(fn `Unlock Spells`
  (bind _returnvalue (subsystem ``))
  (`KismetSystemLibrary.PrintString` "Hello")
  (`/Engine/EditorBlueprintResources/StandardMacros.IsValid` _returnvalue
    (:`Is Valid`
      (for _array_element (`self.unlockID`)
        (`self.UnlockSpell` _returnvalue _array_element)
        (remove `self.OnInteract` (`|CreateDelegate` :!event `Unlock Spells`) :!label _label)))
    (:`Is Not Valid`
      _))
  (goto _label))

(fn `UserConstructionScript`)