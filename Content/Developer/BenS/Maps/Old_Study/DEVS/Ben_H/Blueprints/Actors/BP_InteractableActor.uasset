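; BP_InteractableActor is an interactable actor, apparently meant as a base class, that shows an optional interaction prompt.
; When HasUI is set, InRange creates a screen-space widget from GetImage and GetText, attached to the component GetInteractText returns.
; InRangeExited plays the Appear animation in reverse, then destroys the widget component after a short delay.
; The getters return placeholder defaults: empty text, no image, and the root component as anchor.
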(event `self.InRange`
  (params (Player :type "Object Object Reference"))
  (if (`self.HasUI`)
    (`self.InteractionWidgetComponent`
      (:`then`)
      (:`else`
        (bind _returnvalue (`|CreateWidget` null null (`self.GetImage`) (`self.GetText`)))
        (bind _output_get (set `self.Interact` _returnvalue))
        (bind _returnvalue_2 (`AddComponent|NODE_AddWidgetComponent-0`))
        (bind _output_get_2 (set `self.InteractionWidgetComponent` _returnvalue_2))
        (`WidgetComponent.SetWidget` _output_get_2 _output_get)
        (`WidgetComponent.SetWidgetSpace` _output_get_2 "Screen")
        (`WidgetComponent.SetDrawAtDesiredSize` _output_get_2 true)
        (`PrimitiveComponent.SetCollisionEnabled` _output_get_2 "NoCollision")
        (`SceneComponent.K2_AttachToComponent` _output_get_2 (`self.GetInteractText`) "None" "SnapToTarget" "SnapToTarget" "SnapToTarget" true)))))

(event `self.InRangeExited`
  (params (Player :type "Object Object Reference"))
  (bind _interact (`self.Interact`))
  (if (`self.HasUI`)
    (bind _interactionwidgetcomponent (`self.InteractionWidgetComponent`)
      (:`then`
        (`UserWidget.PlayAnimation` _interact (`/Game/Developer/BenS/Maps/Old_Study/DEVS/Ben_H/Blueprints/Actors/BP_InteractableActor.appear` _interact) 0.0 1 "Reverse" 1.0 false)
        (`KismetSystemLibrary.Delay` 0.2)
        (`ActorComponent.K2_DestroyComponent` _interactionwidgetcomponent))
      (:`else`))))

(fn `GetImage`
  (returns (Image :type "Texture2D Object Reference"))
  (return null))

(fn `GetInteractText`
  (returns (`Attach Component` :type "SceneComponent Object Reference"))
  (return (`self.DefaultSceneRoot`)))

(fn `GetText`
  (returns (Text :type Text))
  (return ""))

(fn `UserConstructionScript`)