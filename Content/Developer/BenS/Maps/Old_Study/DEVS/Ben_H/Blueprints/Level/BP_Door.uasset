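; Interactable door Blueprint that swings open and closed on interaction, provided its HasKey flag is true.
; It binds to OnInteract at BeginPlay, and a FlipFlop alternately plays and reverses a timeline that lerps the whole actor's yaw.
; Getter functions supply the "Door" label and a widget location for interaction prompts, while GetImage returns no image.
; HasKey is only read here, never set.
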(event `self.ReceiveBeginPlay`
  (add `self.OnInteract` (delegate `OnInteract_Event`)))

(event `OnInteract_Event`
  (if (`self.hasKey`)
    (`/Engine/EditorBlueprintResources/StandardMacros.FlipFlop`
      (:`A`
        (bind (_direction _doorrotation) (`Timeline|Timeline` :!label _label)
          (:`Update`
            (`self.K2_SetActorRotation` (`KismetMathLibrary.MakeRotator` 0.0 0.0 (`KismetMathLibrary.Lerp` 90.0 -10.0 _doorrotation))))))
      (:`B`
        (goto _label :!via `Reverse`)))))

(fn `GetImage`
  (returns (Image :type "Texture2D Object Reference"))
  (return null))

(fn `GetInteractText`
  (returns (`Attach Component` :type "SceneComponent Object Reference"))
  (return (`self.WidgetLocation`)))

(fn `GetText`
  (returns (Text :type Text))
  (return "Door"))

(fn `UserConstructionScript`)