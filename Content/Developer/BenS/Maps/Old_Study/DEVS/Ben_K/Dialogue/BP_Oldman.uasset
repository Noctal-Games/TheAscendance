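; BP_Oldman is an interactable old man NPC that cycles through lines of dialogue when the player interacts.
; Entering range attaches a screen-space prompt widget with an icon and text.
; Each interaction creates the WB_Dialogue UI if missing, shows the next Dialogue array entry via PerformDialogue, wrapping after the last, and plays a sound.
; Leaving range reverses the prompt's appear animation, then removes the prompt and dialogue UI.
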(event `self.InRange`
  (params (Player :type "Object Object Reference"))
  (`self.InteractionWidgetComponent`
    (:`then`)
    (:`else`
      (bind _returnvalue (`|CreateWidget` null null (`self.InteractIcon`) (`self.InteractText`)))
      (bind _output_get (set `self.Interact` _returnvalue))
      (bind _returnvalue_2 (`AddComponent|NODE_AddWidgetComponent-0`))
      (bind _output_get_2 (set `self.InteractionWidgetComponent` _returnvalue_2))
      (`WidgetComponent.SetWidget` _output_get_2 _output_get)
      (`WidgetComponent.SetWidgetSpace` _output_get_2 "Screen")
      (`WidgetComponent.SetDrawAtDesiredSize` _output_get_2 true)
      (`PrimitiveComponent.SetCollisionEnabled` _output_get_2 "NoCollision")
      (`SceneComponent.K2_AttachToComponent` _output_get_2 (`self.Scene`) "None" "SnapToTarget" "SnapToTarget" "SnapToTarget" true))))

(event `Create Dialogue`
  (`self.UI`
    (:`then`)
    (:`else`
      (bind _returnvalue (`|CreateWidget` "/Game/Developer/BenS/Maps/Old_Study/DEVS/Ben_K/Dialogue/WB_Dialogue.WB_Dialogue_C" (`GameplayStatics.GetPlayerController` 0)))
      (bind _output_get (set `self.UI` _returnvalue))
      (`UserWidget.AddToViewport` _output_get 0)
      (`TextBlock.SetText` (`/Game/Developer/BenS/Maps/Old_Study/DEVS/Ben_K/Dialogue/WB_Dialogue.TalkText` (`self.UI`)) (`KismetTextLibrary.Conv_StringToText` (`|GetArrayItem` (`self.Dialogue`) (`self.Talkindex`)))))))

(event `self.ReceiveBeginPlay`
  (add `self.OnInteract` (delegate `OnInteract_Event`)))

(event `OnInteract_Event`
  (`|ExecutionSequence`
    (:`then_0`
      (`self.Create Dialogue`))
    (:`then_1`
      (bind _output (`self.PerformDialogue`))
      (`TextBlock.SetText` (`/Game/Developer/BenS/Maps/Old_Study/DEVS/Ben_K/Dialogue/WB_Dialogue.TalkText` (`self.UI`)) _output)
      (`GameplayStatics.PlaySound2D` null 1.0 1.0 0.0 null null))))

(event `self.InRangeExited`
  (params (Player :type "Object Object Reference"))
  (bind _interact (`self.Interact`))
  (bind _interactionwidgetcomponent (`self.InteractionWidgetComponent`)
    (:`then`
      (`UserWidget.PlayAnimation` _interact (`/Game/Developer/BenS/Maps/Old_Study/DEVS/Ben_K/Dialogue/BP_Oldman.appear` _interact) 0.0 1 "Reverse" 1.0 false)
      (`KismetSystemLibrary.Delay` 0.2)
      (`ActorComponent.K2_DestroyComponent` _interactionwidgetcomponent)
      (`Widget.RemoveFromParent` (`self.UI`))
      (set `self.UI` null))
    (:`else`)))

(fn `GetImage`
  (returns (Image :type "Texture2D Object Reference"))
  (return "/Game/Developer/BenS/Maps/Old_Study/DEVS/Ben_K/Dialogue/talk.talk"))

(fn `GetInteractText`
  (returns (`Attach Component` :type "SceneComponent Object Reference"))
  (return (`self.DefaultSceneRoot`)))

(fn `GetText`
  (returns (Text :type Text))
  (return "talk"))

(fn `PerformDialogue`
  (returns (Output :type Text))
  (bind _dialogue (`self.Dialogue`))
  (if (>= (`self.Talkindex`) (- (`KismetArrayLibrary.Array_Length` (`self.Dialogue`)) 1))
    (set `self.Talkindex` 0)
    (return (`KismetTextLibrary.Conv_StringToText` (`|GetArrayItem` _dialogue (`KismetArrayLibrary.Array_LastIndex` _dialogue))))
    (else
      (`/Engine/EditorBlueprintResources/StandardMacros.IncrementInt` (`self.Talkindex`)
        (:`  `
          (return (`KismetTextLibrary.Conv_StringToText` (`|GetArrayItem` (`self.Dialogue`) (- (`self.Talkindex`) 1)))))))))

(fn `UserConstructionScript`)