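; BP_Golem is an interactable golem that plays the Descent cutscene when used.
; On interaction it hides its mesh, removes the player HUD, and runs the LS_Descent level sequence with player input disabled and the player hidden.
; When the sequence finishes, it restores the HUD, swaps to the SM_Golem_2 mesh, shows it again, and spawns an actor at a hardcoded transform.
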(event `self.ReceiveBeginPlay`
  (add `self.OnInteract` (delegate `Interaction`)))

(event `Interaction`
  (`SceneComponent.SetVisibility` (`self.StaticMesh`) false false)
  (bind (_outactor _returnvalue) (`LevelSequencePlayer.CreateLevelSequencePlayer` "/Game/Developer/BenS/Maps/Old_Study/DEVS/Ben_S/Maps/LevelSequence/LS_Descent.LS_Descent" (make `MovieSceneSequencePlaybackSettings` :`bDisableMovementInput` true :`bDisableLookAtInput` true :`bHidePlayer` true)))
  (`MovieSceneSequencePlayer.Play` _returnvalue)
  (`self.RemoveFromViewport` (subsystem ``) 0 (`GameplayStatics.GetPlayerController` 0))
  (add `MovieSceneSequencePlayer.OnFinished` _returnvalue (delegate `OnLevelSequenceEnd`)))

(event `OnLevelSequenceEnd`
  (`self.AddToViewport` (subsystem ``) 0 (`GameplayStatics.GetPlayerController` 0))
  (`StaticMeshComponent.SetStaticMesh` (`self.StaticMesh`) "/Game/Developer/BenS/Maps/Old_Study/DEVS/Ben_S/Maps/GrandLift/Study/Poses/SM_Golem_2.SM_Golem_2")
  (`SceneComponent.SetVisibility` (`self.StaticMesh`) true false)
  (`|SpawnActorFromClass` null (`KismetMathLibrary.MakeTransform` (127.0 1210.0 -832.0) (struct :`Pitch` -80.0)) "Undefined" "MultiplyWithRoot" null null))

(fn `UserConstructionScript`
  (`parent.UserConstructionScript`))