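; BP_ReflectionBook is an interactable book that plays the LS_Reflection level sequence when used.
; On BeginPlay it binds to OnInteract; interaction starts the sequence and disables the book's collision.
; When the sequence finishes, it spawns two actors at hard-coded world transforms and destroys itself.
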(event `self.ReceiveBeginPlay`
  (add `self.OnInteract` (delegate `Interaction`)))

(event `Interaction`
  (bind (_outactor _returnvalue) (`LevelSequencePlayer.CreateLevelSequencePlayer` "/Game/Developer/BenS/Maps/Old_Study/DEVS/Ben_S/Maps/LevelSequence/LS_Reflection.LS_Reflection" (make `MovieSceneSequencePlaybackSettings` :`bHidePlayer` true)))
  (`MovieSceneSequencePlayer.Play` _returnvalue)
  (`PrimitiveComponent.SetCollisionEnabled` (`self.Book`) "NoCollision")
  (add `MovieSceneSequencePlayer.OnFinished` _returnvalue (delegate `OnFinished`)))

(event `OnFinished`
  (`|SpawnActorFromClass` null (`KismetMathLibrary.MakeTransform` (991.0 389.0 87.0) (struct :`Roll` -40.0)) "Undefined" "MultiplyWithRoot" null null)
  (`|SpawnActorFromClass` null (`KismetMathLibrary.MakeTransform` (997.073792 375.0 85.0) (struct :`Yaw` -180.0 :`Roll` 45.0)) "Undefined" "MultiplyWithRoot" null null)
  (`self.K2_DestroyActor`))

(fn `UserConstructionScript`
  (`parent.UserConstructionScript`))