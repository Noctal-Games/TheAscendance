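; BP_Canvas is an interactable canvas in the Study map that plays the LS_Memory sequence the first time it is used.
; BeginPlay binds the interaction event, which runs once to play the sequence with player input and visibility disabled and removes the player HUD.
; When the sequence finishes, it restores the HUD, spawns an actor at a hardcoded location and turns off the canvas's collision.
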(event `self.ReceiveBeginPlay`
  (add `self.OnInteract` (delegate `Interaction`)))

(event `Interaction`
  (`/Engine/EditorBlueprintResources/StandardMacros.DoOnce` false
    (:`Completed`
      (bind (_outactor _returnvalue) (`LevelSequencePlayer.CreateLevelSequencePlayer` "/Game/Developer/BenS/Maps/Old_Study/DEVS/Ben_S/Maps/LevelSequence/LS_Memory.LS_Memory" (make `MovieSceneSequencePlaybackSettings` :`bDisableMovementInput` true :`bDisableLookAtInput` true :`bHidePlayer` true)))
      (`MovieSceneSequencePlayer.Play` _returnvalue)
      (`self.RemoveFromViewport` (subsystem ``) 0 (`GameplayStatics.GetPlayerController` 0))
      (add `MovieSceneSequencePlayer.OnFinished` _returnvalue (delegate `OnSequenceEnd`)))))

(event `OnSequenceEnd`
  (`self.AddToViewport` (subsystem ``) 0 (`GameplayStatics.GetPlayerController` 0))
  (`|SpawnActorFromClass` null (`KismetMathLibrary.MakeTransform` (-2322.0 1083.0 9.0)) "Undefined" "MultiplyWithRoot" null null)
  (`PrimitiveComponent.SetCollisionEnabled` (`self.Canvas`) "NoCollision"))

(fn `UserConstructionScript`
  (`parent.UserConstructionScript`))