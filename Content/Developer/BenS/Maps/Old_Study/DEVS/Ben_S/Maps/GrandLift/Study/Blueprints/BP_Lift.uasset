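; BP_Lift is a lift that carries a character between two fixed heights at a hardcoded world position.
; Standing in the Collision volume for a second fires LiftEvent; leaving early cancels the timer.
; A FlipFlop alternates playing and reversing the LiftMovementDown timeline, which lerps actor height, with a DoOnce blocking retriggers until it finishes.
; During travel, four box colliders are enabled and three VFX components are shown.
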(event `self.collision.OnComponentBeginOverlap`
  (params (OverlappedComponent :type "PrimitiveComponent Object Reference") (OtherActor :type "Actor Object Reference") (OtherComp :type "PrimitiveComponent Object Reference") (OtherBodyIndex :type Integer) (bFromSweep :type Boolean) (SweepResult :type "HitResult Structure (by ref)"))
  (bind _asbp_player_character (cast `` OtherActor))
  (if (== OtherComp (`Character.CapsuleComponent` _asbp_player_character))
    (bind _returnvalue (`KismetSystemLibrary.K2_SetTimerDelegate` (delegate `LiftEvent`) 1.0))
    (set `self.Timer` _returnvalue)))

(event `LiftEvent`
  (`/Engine/EditorBlueprintResources/StandardMacros.DoOnce` false :!label _label
    (:`Completed`
      (`SceneComponent.SetVisibility` (`self.VFX`) true false)
      (`SceneComponent.SetVisibility` (`self.VFX1`) true false)
      (`SceneComponent.SetVisibility` (`self.VFX2`) true false)
      (`/Engine/EditorBlueprintResources/StandardMacros.FlipFlop`
        (:`A`
          (`self.SetCollision` "QueryAndPhysics")
          (bind (_direction _liftlocation) (`Timeline|LiftMovementDown` :!label _label_2)
            (:`Update`
              (`self.K2_SetActorLocation` (`KismetMathLibrary.MakeVector` 2180.0 1080.0 (`KismetMathLibrary.Lerp` 0.0 -890.0 _liftlocation))))
            (:`Finished`
              (`self.SetCollision` "NoCollision")
              (`SceneComponent.SetVisibility` (`self.VFX`) false false)
              (`SceneComponent.SetVisibility` (`self.VFX1`) false false)
              (`SceneComponent.SetVisibility` (`self.VFX2`) false false)
              (goto _label :!via `Reset`))))
        (:`B`
          (`self.SetCollision` "QueryAndPhysics")
          (goto _label_2 :!via `Reverse`))))))

(event `self.collision.OnComponentEndOverlap`
  (params (OverlappedComponent :type "PrimitiveComponent Object Reference") (OtherActor :type "Actor Object Reference") (OtherComp :type "PrimitiveComponent Object Reference") (OtherBodyIndex :type Integer))
  (`KismetSystemLibrary.K2_ClearAndInvalidateTimerHandle` (`self.Timer`)))

(fn `SetCollision`
  (params (NewType :type "ECollisionEnabled Enum" :default "NoCollision"))
  (`PrimitiveComponent.SetCollisionEnabled` (`self.Box`) NewType)
  (`PrimitiveComponent.SetCollisionEnabled` (`self.Box1`) NewType)
  (`PrimitiveComponent.SetCollisionEnabled` (`self.Box2`) NewType)
  (`PrimitiveComponent.SetCollisionEnabled` (`self.Box3`) NewType))

(fn `UserConstructionScript`)