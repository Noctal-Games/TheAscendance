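; Interactable slab door that shows a slate UI widget and, through a separate OpenDoor event, reveals a hidden door.
; The first interaction creates the W_SlabSlate widget; later ones re-show it and remove the player HUD.
; The slate plays an enlarge animation with mouse input enabled, then pauses the game after a short delay.
; OpenDoor destroys the slab component and slides HiddenDoor with two chained timelines, along Y then X.
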(event `self.ReceiveBeginPlay`
  (add `self.OnInteract` (delegate `Interaction`)))

(event `Interaction`
  (bind _returnvalue (`GameplayStatics.GetPlayerController` 0))
  (bind _returnvalue_2 (`GameplayStatics.GetPlayerController` 0))
  (bind _slabslate (`self.SlabSlate`))
  (bind _slabslate_2 (`self.SlabSlate`))
  (bind _asbp_player_character (cast `` (`GameplayStatics.GetPlayerCharacter` 0)))
  (set `self.Player` _asbp_player_character)
  (`|ExecutionSequence`
    (:`then_0`
      (if (`self.FirstInteraction`)
        (bind _returnvalue_3 (`|CreateWidget` "/Game/Developer/BenS/Maps/Old_Study/DEVS/Ben_S/Maps/GrandLift/Study/UI/W_SlabSlate.W_SlabSlate_C"))
        (bind _output_get (set `self.SlabSlate` _returnvalue_3))
        (`UserWidget.AddToViewport` _output_get 0)
        (`WidgetBlueprintLibrary.SetInputMode_GameAndUIEx` _returnvalue_2 null "DoNotLock" false)
        (set `PlayerController.bShowMouseCursor` true _returnvalue_2)
        (bind _asbp_player_character_2 (cast `` (`GameplayStatics.GetPlayerCharacter` 0)))
        (set `self.Player` _asbp_player_character_2)
        (`UserWidget.PlayAnimationForward` _slabslate (`/Game/Developer/BenS/Maps/Old_Study/DEVS/Ben_S/Maps/GrandLift/Study/UI/W_SlabSlate.Enlarge` _slabslate) 1.0 false)
        (`KismetSystemLibrary.Delay` 0.25)
        (`GameplayStatics.SetGamePaused` true)
        (set `self.FirstInteraction` false)))
    (:`then_1`
      (if (not (`self.FirstInteraction`))
        (`self.RemoveFromViewport` (subsystem ``) 0 (`GameplayStatics.GetPlayerController` 0))
        (`Widget.SetVisibility` (`self.SlabSlate`) "Visible")
        (`WidgetBlueprintLibrary.SetInputMode_GameAndUIEx` _returnvalue null "DoNotLock" false)
        (set `PlayerController.bShowMouseCursor` true _returnvalue)
        (bind _asbp_player_character_3 (cast `` (`GameplayStatics.GetPlayerCharacter` 0)))
        (set `self.Player` _asbp_player_character_3)
        (`UserWidget.PlayAnimationForward` _slabslate_2 (`/Game/Developer/BenS/Maps/Old_Study/DEVS/Ben_S/Maps/GrandLift/Study/UI/W_SlabSlate.Enlarge` _slabslate_2) 1.0 false)
        (`KismetSystemLibrary.Delay` 0.25)
        (`GameplayStatics.SetGamePaused` true)))))

(event `OpenDoor`
  (`ActorComponent.K2_DestroyComponent` (`self.Slab`))
  (bind (_direction _doormove) (`Timeline|Movedown`)
    (:`Update`
      (`SceneComponent.K2_SetRelativeLocation` (`self.HiddenDoor`) (`KismetMathLibrary.MakeVector` -100.0 (`KismetMathLibrary.Lerp` 0.0 -10.0 _doormove)) false false))
    (:`Finished`
      (bind (_direction_2 _doormoveleft) (`Timeline|MoveLeft`)
        (:`Update`
          (`SceneComponent.K2_SetRelativeLocation` (`self.HiddenDoor`) (`KismetMathLibrary.MakeVector` (`KismetMathLibrary.Lerp` -100.0 200.0 _doormoveleft) -10.0) false false))))))

(fn `UserConstructionScript`)