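; BP_SlabBench is an interactable bench in the Study map that plays the LS_Stillness cinematic the first time it is used.
; Its OnInteract binding passes through a DoOnce, then plays the sequence with movement and look input disabled and the player hidden, removing the player HUD.
; When the sequence finishes, it restores the HUD and spawns an actor, whose class is unspecified, at a hardcoded world transform.
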(event `self.ReceiveBeginPlay`
  (add `self.OnInteract` (delegate `Interaction`)))

(event `Interaction`
  (`/Engine/EditorBlueprintResources/StandardMacros.DoOnce` false
    (:`Completed`
      (bind (_outactor _returnvalue) (`LevelSequencePlayer.CreateLevelSequencePlayer` "/Game/Developer/BenS/Maps/Old_Study/DEVS/Ben_S/Maps/LevelSequence/LS_Stillness.LS_Stillness" (make `MovieSceneSequencePlaybackSettings` :`bDisableMovementInput` true :`bDisableLookAtInput` true :`bHidePlayer` true)))
      (`MovieSceneSequencePlayer.Play` _returnvalue)
      (`self.RemoveFromViewport` (subsystem ``) 0 (`GameplayStatics.GetPlayerController` 0))
      (add `MovieSceneSequencePlayer.OnFinished` _returnvalue (delegate `OnSequenceEnd`)))))

(event `OnSequenceEnd`
  (`self.AddToViewport` (subsystem ``) 0 (`GameplayStatics.GetPlayerController` 0))
  (`|SpawnActorFromClass` null (`KismetMathLibrary.MakeTransform` (1281.0 1577.0 66.0) (struct :`Pitch` -0.1 :`Yaw` -29.9 :`Roll` 90.099823)) "Undefined" "MultiplyWithRoot" null null))

(fn `UserConstructionScript`
  (`parent.UserConstructionScript`))