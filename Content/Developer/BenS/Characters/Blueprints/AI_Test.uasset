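; AI test character that follows the player while moving with physics-driven animation.
; On BeginPlay it applies physical animation settings from the pelvis down and simulates physics on every body below the pelvis, leaving the pelvis itself unsimulated.
; It then runs AI Move To toward the player character, retrying two seconds after each success or failure.
; A random reachable point lookup is left unused.
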(event `self.ReceiveBeginPlay`
  (bind _mesh (`self.Mesh`))
  (`|ExecutionSequence`
    (:`then_0`
      (`PhysicalAnimationComponent.SetSkeletalMeshComponent` (`self.PhysicalAnimation`) _mesh)
      (`PhysicalAnimationComponent.ApplyPhysicalAnimationSettingsBelow` (`self.PhysicalAnimation`) "pelvis" (make `PhysicalAnimationData` true 250.0 200.0 1000.0 200.0 200.0 200.0) true)
      (`SkeletalMeshComponent.SetAllBodiesBelowSimulatePhysics` _mesh "pelvis" true false))
    (:`then_1`
      (`|AIMoveTo` self (0.0 0.0 0.0) (`CoreFunctionLibrary.GetPlayerCharacter`) 100.0 true :!label _label
        (:`OnSuccess`
          _)
        (:`OnFail`
          _))
      (`KismetSystemLibrary.Delay` 2.0)
      (goto _label))))

(fn `UserConstructionScript`)