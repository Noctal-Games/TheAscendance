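; Test first-person player character that prototypes hand and sword attacks, camera feel and in-range detection.
; Attack inputs branch on WeaponType; sword attacks play montages on the Hands mesh, stepping through combo arrays gated by CanCombo and reset by a retriggerable delay.
; Timelines drive sprint and spell-focus FOV and smooth reorientation, while Tick rolls the camera on fast sprint turns.
; Body mesh hides arm bones and sends overlap range messages through BPI_Player_Functions.
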(event `Key|Five`
  (params (Key :type "Key Structure"))
  ; Test Animation cycle
  (:`Pressed`
    (`|PlayMontage` (`self.Hands`) "/Game/Developer/BenS/Animation/Locomotion/Montages/Spell/1H/Offhand/Projectile/AMO_Projectile_Instantaneous.AMO_Projectile_Instantaneous")))

(event `Key|Six`
  (params (Key :type "Key Structure"))
  ; Test Animation cycle
  (:`Pressed`
    (`|PlayMontage` (`self.Hands`) "/Game/Developer/BenS/Animation/Locomotion/Montages/Spell/1H/MainHand/Projectile/AM_Projectile_Instantaneous.AM_Projectile_Instantaneous")))

(event `PlayerFocus`
  ; Zooms in 3 degrees when firing a spell
  (bind (_direction _camerafov) (`Timeline|CameraFocus` :!label _label)
    (:`Update`
      (`CameraComponent.SetFieldOfView` (`self.m_Camera`) (`KismetMathLibrary.Lerp` 100.0 97.0 _camerafov)))))

(event `PlayerReleaseFocus`
  ; Test Camera shake
  (`GameplayStatics.PlayWorldCameraShake` "/Game/Developer/BenS/GameFeel/Camera/Spell/Instantaneous.Instantaneous_C" (`PlayerCameraManager.GetCameraLocation` (`GameplayStatics.GetPlayerCameraManager` 0)) 0.0 10.0)
  (goto _label :!via `Reverse`))

(event `self.ReceiveTick`
  (params (DeltaSeconds :type "Float (single-precision)"))
  ; Camera Lean when sprinting and turning very fast
  (`self.CameraLean` (`self.GetInputAxisKeyValue`)))

(event `EnhancedInput|/Game/TheAscendance/Input/Gameplay/IA_Sprint`
  (params (ActionValue :type Boolean) (ElapsedSeconds :type "Float (double-precision)") (TriggeredSeconds :type "Float (double-precision)") (InputAction :type "InputAction Object Reference" :default "/Game/TheAscendance/Input/Gameplay/IA_Sprint.IA_Sprint"))
  ; Chnaged FOV when sprinting
  (:`Triggered`
    (if (> (`KismetMathLibrary.VSize` (`MovementComponent.Velocity` (`self.CharacterMovement`))) 601.0)
      (bind (_direction _camerafov) (`Timeline|CameraFovChange` :!label _label_2)
        (:`Update`
          (`CameraComponent.SetFieldOfView` (`self.m_Camera`) (`KismetMathLibrary.Lerp` 100.0 120.0 _camerafov))))
      (else
        (goto _label_2 :!via `Reverse`))))
  (:`Completed`
    (goto _label_2 :!via `Reverse`)))

(event `EnhancedInput|/Game/TheAscendance/Input/Gameplay/IA_MainHandPrimaryAttack`
  (params (ActionValue :type Boolean) (ElapsedSeconds :type "Float (double-precision)") (TriggeredSeconds :type "Float (double-precision)") (InputAction :type "InputAction Object Reference" :default "/Game/TheAscendance/Input/Gameplay/IA_MainHandPrimaryAttack.IA_MainHandPrimaryAttack"))
  ; Switches to events based on held item
  (:`Triggered`
    (switch `EWeaponType` (`self.WeaponType`)
      (:`HAND`
        (`self.MainHandPrimaryHand`))
      (:`SWORD`
        (`self.MainHandPrimarySword`)))))

(event `MainHandPrimarySword`
  ; Combo attack set up: goes up an index when 'CanCombo' is true, index resets when either time passed and hasnt been retriggered or its the end of the combo index
  (bind _returnvalue (`self.IsMainHandAttacking`))
  (if _returnvalue
    (if (`self.CanCombo`)
      (bind _animation (`self.MainHandCombo`))
      (`|PlayMontage` (`self.Hands`) _animation
        (:`then`
          (set `self.CanCombo` false))))))

(event `EnhancedInput|/Game/TheAscendance/Input/Gameplay/IA_OffhandPrimaryAttack`
  (params (ActionValue :type Boolean) (ElapsedSeconds :type "Float (double-precision)") (TriggeredSeconds :type "Float (double-precision)") (InputAction :type "InputAction Object Reference" :default "/Game/TheAscendance/Input/Gameplay/IA_OffhandPrimaryAttack.IA_OffhandPrimaryAttack"))
  ; Switches to events based on held item
  (:`Triggered`
    (switch `EWeaponType` (`self.WeaponType`)
      (:`HAND`
        (`self.OffhandPrimaryHand`))
      (:`SWORD`
        (`self.OffhandPrimarySword`)))))

(event `OffhandPrimarySword`
  ; Combo attack set up: goes up an index when 'CanCombo' is true, index resets when either time passed and hasnt been retriggered or its the end of the combo index
  (bind _returnvalue (`self.IsOffhandAttacking`))
  (if _returnvalue
    (if (`self.CanCombo`)
      (bind _animation (`self.OffhandCombo`))
      (`|PlayMontage` (`self.Hands`) _animation
        (:`then`
          (set `self.CanCombo` false))))))

(event `MainHandAltSword`
  ; Combo attack set up: goes up an index when 'CanCombo' is true, index resets when either time passed and hasnt been retriggered or its the end of the combo index
  (bind _returnvalue (`self.IsMainHandAttacking`))
  (if _returnvalue
    (`|PlayMontage` (`self.Hands`) "/Game/Developer/BenS/Animation/Locomotion/Montages/Melee/MainHand/AM_Alt_Attack.AM_Alt_Attack")))

(event `EnhancedInput|/Game/TheAscendance/Input/Gameplay/IA_MainHandAltAttack`
  (params (ActionValue :type Boolean) (ElapsedSeconds :type "Float (double-precision)") (TriggeredSeconds :type "Float (double-precision)") (InputAction :type "InputAction Object Reference" :default "/Game/TheAscendance/Input/Gameplay/IA_MainHandAltAttack.IA_MainHandAltAttack"))
  ; Switches to events based on held item
  (:`Triggered`
    (switch `EWeaponType` (`self.WeaponType`)
      (:`SWORD`
        (`self.MainHandAltSword`)))))

(event `ContinueCombo`
  ; Combo attack set up: goes up an index when 'CanCombo' is true, index resets when either time passed and hasnt been retriggered or its the end of the combo index
  (`/Engine/EditorBlueprintResources/StandardMacros.IncrementInt` (`self.ComboIndex`)
    (:`  `
      (`KismetSystemLibrary.RetriggerableDelay` 1.0)
      (set `self.ComboIndex` 0 :!label _label_3))))

(event `ResetCombo`
  ; Combo attack set up: goes up an index when 'CanCombo' is true, index resets when either time passed and hasnt been retriggered or its the end of the combo index
  (goto _label_3))

(event `OffhandAltSword`
  ; Combo attack set up: goes up an index when 'CanCombo' is true, index resets when either time passed and hasnt been retriggered or its the end of the combo index
  (bind _returnvalue (`self.IsOffhandAttacking`))
  (if _returnvalue
    (`|PlayMontage` (`self.Hands`) "/Game/Developer/BenS/Animation/Locomotion/Montages/Melee/Offhand/AMO_Alt_Attack.AMO_Alt_Attack")))

(event `EnhancedInput|/Game/TheAscendance/Input/Gameplay/IA_OffhandAltAttack`
  (params (ActionValue :type Boolean) (ElapsedSeconds :type "Float (double-precision)") (TriggeredSeconds :type "Float (double-precision)") (InputAction :type "InputAction Object Reference" :default "/Game/TheAscendance/Input/Gameplay/IA_OffhandAltAttack.IA_OffhandAltAttack"))
  ; Switches to events based on held item
  (:`Triggered`
    (switch `EWeaponType` (`self.WeaponType`)
      (:`SWORD`
        (`self.OffhandAltSword`)))))

(event `SmoothOrientation`
  (params (NewControlRotation :type "Rotator Structure"))
  (bind _initialcontrolrotation (`self.InitialControlRotation`))
  ; Orientates the player if the control rotation or world rotation are not 0, it takes track of the initial rotation then resets it on the timeline for a smooth rotation
  (if (or (!= (.roll (`Controller.GetControlRotation` (`GameplayStatics.GetPlayerController` 0))) 0.0) (!= (.roll (`SceneComponent.K2_GetComponentRotation` (`self.CapsuleComponent`))) 0.0))
    (set `self.InitialControlRotation` (`Controller.GetControlRotation` (`GameplayStatics.GetPlayerController` 0)))
    (set `self.InitialWorldRotation` (`SceneComponent.K2_GetComponentRotation` (`self.CapsuleComponent`)))
    (bind (_direction _alpha) (`Timeline|RotatePlayer` :!via `PlayFromStart`)
      (:`Update`
        (`Controller.SetControlRotation` (`GameplayStatics.GetPlayerController` 0) (`|EaseFunction` "EaseInOut" _alpha _initialcontrolrotation (`KismetMathLibrary.MakeRotator` 0.0 (.pitch _initialcontrolrotation) (.yaw _initialcontrolrotation))))
        (`SceneComponent.K2_SetWorldRotation` (`self.CapsuleComponent`) (`|EaseFunction` "EaseInOut" _alpha (`self.InitialWorldRotation`) (`KismetMathLibrary.MakeRotator` 0.0)) false false)))))

(event `MainHandPrimaryHand`
  (bind _returnvalue (`self.IsMainHandAttacking`))
  (if _returnvalue
    (`/Engine/EditorBlueprintResources/StandardMacros.IncrementInt` (`self.SomaticIndex`)
      (:`  `
        (`KismetSystemLibrary.Delay` 0.1)
        (`/Engine/EditorBlueprintResources/StandardMacros.IncrementInt` (`self.SomaticIndex`)
          (:`  `
            (`KismetSystemLibrary.Delay` 0.1)
            (`/Engine/EditorBlueprintResources/StandardMacros.IncrementInt` (`self.SomaticIndex`)
              (:`  `
                (`KismetSystemLibrary.Delay` 0.1)
                (set `self.SomaticIndex` 0)))))))))

(event `OffhandPrimaryHand`
  (bind _returnvalue (`self.IsOffhandAttacking`))
  (if _returnvalue
    _))

(event `self.Mesh.OnComponentBeginOverlap`
  (params (OverlappedComponent :type "PrimitiveComponent Object Reference") (OtherActor :type "Actor Object Reference") (OtherComp :type "PrimitiveComponent Object Reference") (OtherBodyIndex :type Integer) (bFromSweep :type Boolean) (SweepResult :type "HitResult Structure (by ref)"))
  ; In Range and Out of range set up
  (if (`KismetSystemLibrary.DoesImplementInterface` OtherActor "/Game/Developer/BenS/Interfaces/BPI_Player_Functions.BPI_Player_Functions_C")
    (message `/Game/Developer/BenS/Interfaces/BPI_Player_Functions.InRange` OtherActor self)))

(event `self.Mesh.OnComponentEndOverlap`
  (params (OverlappedComponent :type "PrimitiveComponent Object Reference") (OtherActor :type "Actor Object Reference") (OtherComp :type "PrimitiveComponent Object Reference") (OtherBodyIndex :type Integer))
  ; In Range and Out of range set up
  (if (`KismetSystemLibrary.DoesImplementInterface` OtherActor "/Game/Developer/BenS/Interfaces/BPI_Player_Functions.BPI_Player_Functions_C")
    (message `/Game/Developer/BenS/Interfaces/BPI_Player_Functions.OutRange` OtherActor self)))

(fn `CameraLean`
  (params (ScaleVal :type "Float (double-precision)"))
  (locals (LeanSpeed :type "Float (double-precision)" :default 2.0) (LeanAngle :type "Float (double-precision)" :default 5.0))
  (bind (_returnvalue_roll _returnvalue_pitch _returnvalue_yaw) (`KismetMathLibrary.BreakRotator` (`self.GetControlRotation`)))
  (bind (_returnvalue_roll_2 _returnvalue_pitch_2 _returnvalue_yaw_2) (`KismetMathLibrary.BreakRotator` (`self.GetControlRotation`)))
  (bind (_returnvalue_roll_3 _returnvalue_pitch_3 _returnvalue_yaw_3) (`KismetMathLibrary.BreakRotator` (`self.GetControlRotation`)))
  (bind _charactermovement (`self.CharacterMovement`))
  (if (and (> (`KismetMathLibrary.VSize` (`MovementComponent.Velocity` _charactermovement)) 601.0) (not (`NavMovementInterface.IsFalling` _charactermovement)) (!= (`local.ScaleVal`) 0.0))
    (if (> (`local.ScaleVal`) 3.0)
      (`Controller.SetControlRotation` (`GameplayStatics.GetPlayerController` 0) (`KismetMathLibrary.RInterpTo` (`self.GetControlRotation`) (`KismetMathLibrary.MakeRotator` (`local.LeanAngle`) _returnvalue_pitch_2 _returnvalue_yaw_2) (`GameplayStatics.GetWorldDeltaSeconds`) (`local.LeanSpeed`)))
      (elif (< (`local.ScaleVal`) -3.0)
        (`Controller.SetControlRotation` (`GameplayStatics.GetPlayerController` 0) (`KismetMathLibrary.RInterpTo` (`self.GetControlRotation`) (`KismetMathLibrary.MakeRotator` (- 360.0 (`local.LeanAngle`)) _returnvalue_pitch_3 _returnvalue_yaw_3) (`GameplayStatics.GetWorldDeltaSeconds`) (`local.LeanSpeed`)))))
    (else
      (`Controller.SetControlRotation` (`GameplayStatics.GetPlayerController` 0) (`KismetMathLibrary.RInterpTo` (`self.GetControlRotation`) (`KismetMathLibrary.MakeRotator` 0.0 _returnvalue_pitch _returnvalue_yaw) (`GameplayStatics.GetWorldDeltaSeconds`) (`local.LeanSpeed`))))))

(fn `GetHandSwayData`
  (returns (sideMovement :type "Float (double-precision)") (X :type "Float (double-precision)") (Y :type "Float (double-precision)"))
  (bind _returnvalue_x (`KismetMathLibrary.BreakVector2D` (`|GetInputActionValue`)))
  (return _returnvalue_x (`self.GetInputAxisKeyValue`) (`self.GetInputAxisKeyValue`)))

(fn `MainHandCombo`
  (returns (animation :type "AnimMontage Object Reference"))
  (bind _mainhandattacks (`self.MainHandAttacks`))
  (if (>= (`self.ComboIndex`) (- (`KismetArrayLibrary.Array_Length` (`self.MainHandAttacks`)) 1))
    (`self.ResetCombo`)
    (return (`|GetArrayItem` _mainhandattacks (`KismetArrayLibrary.Array_LastIndex` _mainhandattacks)))
    (else
      (`self.ContinueCombo`)
      (return (`|GetArrayItem` (`self.MainHandAttacks`) (- (`self.ComboIndex`) 1))))))

(fn `MontageShowcase`
  (params (Montage :type "Array of AnimMontage Object Reference (by ref)"))
  (returns (animation :type "AnimMontage Object Reference"))
  (if (not (>= (`self.MontageIndex`) (- (`KismetArrayLibrary.Array_Length` Montage) 1)))
    (`/Engine/EditorBlueprintResources/StandardMacros.IncrementInt` (`self.MontageIndex`)
      (:`  `
        (return (`|GetArrayItem` Montage (- (`self.MontageIndex`) 1)))))))

(fn `OffhandCombo`
  (returns (animation :type "AnimMontage Object Reference"))
  (bind _offhand_attacks (`self.Offhand Attacks`))
  (if (>= (`self.ComboIndex`) (- (`KismetArrayLibrary.Array_Length` (`self.Offhand Attacks`)) 1))
    (`self.ResetCombo`)
    (return (`|GetArrayItem` _offhand_attacks (`KismetArrayLibrary.Array_LastIndex` _offhand_attacks)))
    (else
      (`self.ContinueCombo`)
      (return (`|GetArrayItem` (`self.Offhand Attacks`) (- (`self.ComboIndex`) 1))))))

(fn `UserConstructionScript`
  (for _array_element (`self.ArmBones`)
    (`SkinnedMeshComponent.HideBoneByName` (`self.Mesh`) _array_element "PBO_None")))