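; MyBaseEnemy is an enemy character Blueprint that wanders randomly with a physically animated body.
; On BeginPlay it applies physical animation settings from the pelvis down and simulates physics on the bodies below the pelvis, leaving the pelvis itself unsimulated.
; It then loops AI Move To toward random reachable points around its current location, retrying after a short delay whether the move succeeds or fails.
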(event `self.ReceiveBeginPlay`
  (`|ExecutionSequence`
    (:`then_0`
      (`PhysicalAnimationComponent.SetSkeletalMeshComponent` (`self.PhysicalAnimation`) (`self.Mesh`))
      (`PhysicalAnimationComponent.ApplyPhysicalAnimationSettingsBelow` (`self.PhysicalAnimation`) "pelvis" (make `PhysicalAnimationData` true 1000.0 100.0 1000.0 100.0 100.0 100.0) true)
      (`SkeletalMeshComponent.SetAllBodiesBelowSimulatePhysics` (`self.Mesh`) "pelvis" true false))
    (:`then_1`
      (`|AIMoveTo` self (`NavigationSystemV1.K2_GetRandomReachablePointInRadius` (`self.K2_GetActorLocation`) 500.0 null null) null :!label _label
        (:`OnSuccess`
          _)
        (:`OnFail`
          _))
      (`KismetSystemLibrary.Delay` 0.2)
      (goto _label))))

(fn `UserConstructionScript`)