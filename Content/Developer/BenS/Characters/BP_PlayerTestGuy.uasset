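; First-person player test character with separate hands and body mesh arm bones hidden, handling melee attacks, camera feel and interaction.
; Main and offhand inputs play montages on the hands, with primary attacks gated by CanCombo and stepping a shared index that resets after a retriggerable delay or final hit.
; Timelines shift FOV for spell focus and sprinting, while Tick rolls control rotation during fast turns.
; Interaction and range notifications reach overlapping actors through BPI_PlayerInteract.
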(event `self.ReceiveBeginPlay`
  ; Hides arms at the beginning
  (for _array_element (`self.ArmBones`)
    (`SkinnedMeshComponent.HideBoneByName` (`self.Mesh`) _array_element "PBO_None")))

(event `PlayerFocus`
  ; Zooms in 3 degrees when firing a spell
  (bind (_direction _camerafov) (`Timeline|CameraFocus` :!label _label)
    (:`Update`
      (`CameraComponent.SetFieldOfView` (`self.m_Camera`) (`KismetMathLibrary.Lerp` 100.0 97.0 _camerafov)))))

(event `PlayerReleaseFocus`
  ; Zooms in 3 degrees when firing a spell
  (goto _label :!via `Reverse`))

(event `self.ReceiveTick`
  (params (DeltaSeconds :type "Float (single-precision)"))
  ; Camera Lean when sprinting and turning very fast
  (`self.CameraLean` (`self.GetInputAxisKeyValue`)))

(event `EnhancedInput|/Game/TheAscendance/Input/IA_Sprint`
  (params (ActionValue :type Boolean) (ElapsedSeconds :type "Float (double-precision)") (TriggeredSeconds :type "Float (double-precision)") (InputAction :type "InputAction Object Reference" :default "/Game/TheAscendance/Input/IA_Sprint.IA_Sprint"))
  ; Chnaged FOV when sprinting
  (:`Triggered`
    (if (> (`KismetMathLibrary.VSize` (`MovementComponent.Velocity` (`self.CharacterMovement`))) 601.0)
      (bind (_direction _camerafov) (`Timeline|CameraFovChange` :!label _label_2)
        (:`Update`
          (`CameraComponent.SetFieldOfView` (`self.m_Camera`) (`KismetMathLibrary.Lerp` 100.0 120.0 _camerafov))))
      (else
        (goto _label_2 :!via `Reverse`))))
  (:`Completed`
    (goto _label_2 :!via `Reverse`)))

(event `EnhancedInput|/Game/TheAscendance/Input/IA_MainHandPrimaryAttack`
  (params (ActionValue :type Boolean) (ElapsedSeconds :type "Float (double-precision)") (TriggeredSeconds :type "Float (double-precision)") (InputAction :type "InputAction Object Reference" :default "/Game/TheAscendance/Input/IA_MainHandPrimaryAttack.IA_MainHandPrimaryAttack"))
  ; Combo attack set up: goes up an index when 'CanCombo' is true, index resets when either time passed and hasnt been retriggered or its the end of the combo index
  (:`Triggered`
    (bind _returnvalue (`self.IsMainHandAttacking`))
    (if _returnvalue
      (if (`self.CanCombo`)
        (bind _animation (`self.MainHandCombo`))
        (`|PlayMontage` (`self.Hands`) _animation
          (:`then`
            (set `self.CanCombo` false)))))))

(event `EnhancedInput|/Game/TheAscendance/Input/IA_OffhandPrimaryAttack`
  (params (ActionValue :type Boolean) (ElapsedSeconds :type "Float (double-precision)") (TriggeredSeconds :type "Float (double-precision)") (InputAction :type "InputAction Object Reference" :default "/Game/TheAscendance/Input/IA_OffhandPrimaryAttack.IA_OffhandPrimaryAttack"))
  ; Combo attack set up: goes up an index when 'CanCombo' is true, index resets when either time passed and hasnt been retriggered or its the end of the combo index
  (:`Triggered`
    (bind _returnvalue (`self.IsOffhandAttacking`))
    (if _returnvalue
      (if (`self.CanCombo`)
        (bind _animation (`self.OffhandCombo`))
        (`|PlayMontage` (`self.Hands`) _animation
          (:`then`
            (set `self.CanCombo` false)))))))

(event `EnhancedInput|/Game/TheAscendance/Input/IA_MainHandAltAttack`
  (params (ActionValue :type Boolean) (ElapsedSeconds :type "Float (double-precision)") (TriggeredSeconds :type "Float (double-precision)") (InputAction :type "InputAction Object Reference" :default "/Game/TheAscendance/Input/IA_MainHandAltAttack.IA_MainHandAltAttack"))
  ; Combo attack set up: goes up an index when 'CanCombo' is true, index resets when either time passed and hasnt been retriggered or its the end of the combo index
  (:`Triggered`
    (bind _returnvalue (`self.IsMainHandAttacking`))
    (if _returnvalue
      (`|PlayMontage` (`self.Hands`) "/Game/Developer/BenS/Animation/Locomotion/Montages/AM_Alt_Attack.AM_Alt_Attack"))))

(event `ContinueCombo`
  ; Combo attack set up: goes up an index when 'CanCombo' is true, index resets when either time passed and hasnt been retriggered or its the end of the combo index
  (`/Engine/EditorBlueprintResources/StandardMacros.IncrementInt` (`self.ComboIndex`)
    (:`  `
      (`KismetSystemLibrary.RetriggerableDelay` 1.0)
      (set `self.ComboIndex` 0 :!label _label_3))))

(event `ResetCombo`
  ; Combo attack set up: goes up an index when 'CanCombo' is true, index resets when either time passed and hasnt been retriggered or its the end of the combo index
  (goto _label_3))

(event `EnhancedInput|/Game/TheAscendance/Input/IA_OffhandAltAttack`
  (params (ActionValue :type Boolean) (ElapsedSeconds :type "Float (double-precision)") (TriggeredSeconds :type "Float (double-precision)") (InputAction :type "InputAction Object Reference" :default "/Game/TheAscendance/Input/IA_OffhandAltAttack.IA_OffhandAltAttack"))
  ; Combo attack set up: goes up an index when 'CanCombo' is true, index resets when either time passed and hasnt been retriggered or its the end of the combo index
  (:`Triggered`
    (bind _returnvalue (`self.IsOffhandAttacking`))
    (if _returnvalue
      (`|PlayMontage` (`self.Hands`) "/Game/Developer/BenS/Animation/Locomotion/Montages/AMO_Alt_Attack.AMO_Alt_Attack"))))

(event `EnhancedInput|/Game/TheAscendance/Input/IA_Interact`
  (params (ActionValue :type Boolean) (ElapsedSeconds :type "Float (double-precision)") (TriggeredSeconds :type "Float (double-precision)") (InputAction :type "InputAction Object Reference" :default "/Game/TheAscendance/Input/IA_Interact.IA_Interact"))
  ; Basic Interact system
  (:`Triggered`
    (for _array_element (`PrimitiveComponent.GetOverlappingActors` (`self.CapsuleComponent`) "/Script/Engine.Actor")
      (if (`KismetSystemLibrary.DoesImplementInterface` _array_element "/Game/Developer/BenS/Interfaces/BPI_PlayerInteract.BPI_PlayerInteract_C")
        (message `/Game/Developer/BenS/Interfaces/BPI_PlayerInteract.OnInteract` _array_element)))))

(event `self.Mesh.OnComponentBeginOverlap`
  (params (OverlappedComponent :type "PrimitiveComponent Object Reference") (OtherActor :type "Actor Object Reference") (OtherComp :type "PrimitiveComponent Object Reference") (OtherBodyIndex :type Integer) (bFromSweep :type Boolean) (SweepResult :type "HitResult Structure (by ref)"))
  ; Basic Interact system
  (if (`KismetSystemLibrary.DoesImplementInterface` OtherActor "/Game/Developer/BenS/Interfaces/BPI_PlayerInteract.BPI_PlayerInteract_C")
    (message `/Game/Developer/BenS/Interfaces/BPI_PlayerInteract.InRange` OtherActor self)))

(event `self.Mesh.OnComponentEndOverlap`
  (params (OverlappedComponent :type "PrimitiveComponent Object Reference") (OtherActor :type "Actor Object Reference") (OtherComp :type "PrimitiveComponent Object Reference") (OtherBodyIndex :type Integer))
  ; Basic Interact system
  (if (`KismetSystemLibrary.DoesImplementInterface` OtherActor "/Game/Developer/BenS/Interfaces/BPI_PlayerInteract.BPI_PlayerInteract_C")
    (message `/Game/Developer/BenS/Interfaces/BPI_PlayerInteract.OutRange` OtherActor self)))

(fn `CameraLean`
  (params (ScaleVal :type "Float (double-precision)"))
  (locals (LeanSpeed :type "Float (double-precision)" :default 2.0) (LeanAngle :type "Float (double-precision)" :default 5.0))
  (bind (_returnvalue_roll _returnvalue_pitch _returnvalue_yaw) (`KismetMathLibrary.BreakRotator` (`self.GetControlRotation`)))
  (bind (_returnvalue_roll_2 _returnvalue_pitch_2 _returnvalue_yaw_2) (`KismetMathLibrary.BreakRotator` (`self.GetControlRotation`)))
  (bind (_returnvalue_roll_3 _returnvalue_pitch_3 _returnvalue_yaw_3) (`KismetMathLibrary.BreakRotator` (`self.GetControlRotation`)))
  (bind _charactermovement (`self.CharacterMovement`))
  (if (and (> (`KismetMathLibrary.VSize` (`MovementComponent.Velocity` _charactermovement)) 601.0) (not (`NavMovementInterface.IsFalling` _charactermovement)) (!= (`local.ScaleVal`) 0.0))
    (if (> (`local.ScaleVal`) 3.0)
      (`Controller.SetControlRotation` (`GameplayStatics.GetPlayerController` 0) (`KismetMathLibrary.RInterpTo` (`self.GetControlRotation`) (`KismetMathLibrary.MakeRotator` (`local.LeanAngle`) _returnvalue_pitch_2 _returnvalue_yaw_2) (`GameplayStatics.GetWorldDeltaSeconds`) (`local.LeanSpeed`)))
      (elif (< (`local.ScaleVal`) -3.0)
        (`Controller.SetControlRotation` (`GameplayStatics.GetPlayerController` 0) (`KismetMathLibrary.RInterpTo` (`self.GetControlRotation`) (`KismetMathLibrary.MakeRotator` (- 360.0 (`local.LeanAngle`)) _returnvalue_pitch_3 _returnvalue_yaw_3) (`GameplayStatics.GetWorldDeltaSeconds`) (`local.LeanSpeed`)))))
    (else
      (`Controller.SetControlRotation` (`GameplayStatics.GetPlayerController` 0) (`KismetMathLibrary.RInterpTo` (`self.GetControlRotation`) (`KismetMathLibrary.MakeRotator` 0.0 _returnvalue_pitch _returnvalue_yaw) (`GameplayStatics.GetWorldDeltaSeconds`) (`local.LeanSpeed`))))))

(fn `GetHandSwayData`
  (returns (sideMovement :type "Float (double-precision)") (X :type "Float (double-precision)") (Y :type "Float (double-precision)"))
  (bind _returnvalue_x (`KismetMathLibrary.BreakVector2D` (`|GetInputActionValue`)))
  (return _returnvalue_x (`self.GetInputAxisKeyValue`) (`self.GetInputAxisKeyValue`)))

(fn `MainHandCombo`
  (returns (animation :type "AnimMontage Object Reference"))
  (bind _mainhandattacks (`self.MainHandAttacks`))
  (if (>= (`self.ComboIndex`) (- (`KismetArrayLibrary.Array_Length` (`self.MainHandAttacks`)) 1))
    (`self.ResetCombo`)
    (return (`|GetArrayItem` _mainhandattacks (`KismetArrayLibrary.Array_LastIndex` _mainhandattacks)))
    (else
      (`self.ContinueCombo`)
      (return (`|GetArrayItem` (`self.MainHandAttacks`) (- (`self.ComboIndex`) 1))))))

(fn `OffhandCombo`
  (returns (animation :type "AnimMontage Object Reference"))
  (bind _offhand_attacks (`self.Offhand Attacks`))
  (if (>= (`self.ComboIndex`) (- (`KismetArrayLibrary.Array_Length` (`self.Offhand Attacks`)) 1))
    (`self.ResetCombo`)
    (return (`|GetArrayItem` _offhand_attacks (`KismetArrayLibrary.Array_LastIndex` _offhand_attacks)))
    (else
      (`self.ContinueCombo`)
      (return (`|GetArrayItem` (`self.Offhand Attacks`) (- (`self.ComboIndex`) 1))))))

(fn `UserConstructionScript`)