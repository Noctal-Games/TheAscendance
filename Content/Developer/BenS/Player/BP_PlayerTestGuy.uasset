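; Test player character Blueprint that adds speed-based camera feedback and hides the mesh's arm bones at BeginPlay.
; Sprint input plays a timeline that widens camera FOV at high speed, reversing it on slowdown or release.
; Tick feeds an input axis into CameraLean, which interpolates control-rotation roll for fast grounded turns and levels it when slow, airborne or input is zero.
; GetHandSwayData exposes move and axis input for hand sway.
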(event `EnhancedInput|/Game/TheAscendance/Input/IA_Sprint`
  (params (ActionValue :type Boolean) (ElapsedSeconds :type "Float (double-precision)") (TriggeredSeconds :type "Float (double-precision)") (InputAction :type "InputAction Object Reference" :default "/Game/TheAscendance/Input/IA_Sprint.IA_Sprint"))
  (:`Triggered`
    (if (> (`KismetMathLibrary.VSize` (`MovementComponent.Velocity` (`self.CharacterMovement`))) 601.0)
      (bind (_direction _camerafov) (`Timeline|CameraFovChange` :!label _label)
        (:`Update`
          (`CameraComponent.SetFieldOfView` (`self.m_Camera`) (`KismetMathLibrary.Lerp` 100.0 120.0 _camerafov))))
      (else
        (goto _label :!via `Reverse`))))
  (:`Completed`
    (goto _label :!via `Reverse`)))

(event `self.ReceiveTick`
  (params (DeltaSeconds :type "Float (single-precision)"))
  (`self.CameraLean` (`self.GetInputAxisKeyValue`)))

(event `self.ReceiveBeginPlay`
  (`|ExecutionSequence`
    (:`then_0`
      (for _array_element (`self.ArmBones`)
        (`SkinnedMeshComponent.HideBoneByName` (`self.Mesh`) _array_element "PBO_None")))))

(fn `CameraLean`
  (params (ScaleVal :type "Float (double-precision)"))
  (locals (LeanSpeed :type "Float (double-precision)" :default 2.0) (LeanAngle :type "Float (double-precision)" :default 6.0))
  (bind (_returnvalue_roll _returnvalue_pitch _returnvalue_yaw) (`KismetMathLibrary.BreakRotator` (`self.GetControlRotation`)))
  (bind (_returnvalue_roll_2 _returnvalue_pitch_2 _returnvalue_yaw_2) (`KismetMathLibrary.BreakRotator` (`self.GetControlRotation`)))
  (bind (_returnvalue_roll_3 _returnvalue_pitch_3 _returnvalue_yaw_3) (`KismetMathLibrary.BreakRotator` (`self.GetControlRotation`)))
  (bind _charactermovement (`self.CharacterMovement`))
  (if (and (> (`KismetMathLibrary.VSize` (`MovementComponent.Velocity` _charactermovement)) 601.0) (not (`NavMovementInterface.IsFalling` _charactermovement)) (!= (`local.ScaleVal`) 0.0))
    (if (> (`local.ScaleVal`) 3.0)
      (`Controller.SetControlRotation` (`GameplayStatics.GetPlayerController` 0) (`KismetMathLibrary.RInterpTo` (`self.GetControlRotation`) (`KismetMathLibrary.MakeRotator` (`local.LeanAngle`) _returnvalue_pitch_2 _returnvalue_yaw_2) (`GameplayStatics.GetWorldDeltaSeconds`) (`local.LeanSpeed`)))
      (elif (< (`local.ScaleVal`) -3.0)
        (`Controller.SetControlRotation` (`GameplayStatics.GetPlayerController` 0) (`KismetMathLibrary.RInterpTo` (`self.GetControlRotation`) (`KismetMathLibrary.MakeRotator` (- 360.0 (`local.LeanAngle`)) _returnvalue_pitch_3 _returnvalue_yaw_3) (`GameplayStatics.GetWorldDeltaSeconds`) (`local.LeanSpeed`)))))
    (else
      (`Controller.SetControlRotation` (`GameplayStatics.GetPlayerController` 0) (`KismetMathLibrary.RInterpTo` (`self.GetControlRotation`) (`KismetMathLibrary.MakeRotator` 0.0 _returnvalue_pitch _returnvalue_yaw) (`GameplayStatics.GetWorldDeltaSeconds`) (`local.LeanSpeed`))))))

(fn `GetHandSwayData`
  (returns (sideMovement :type "Float (double-precision)") (X :type "Float (double-precision)") (Y :type "Float (double-precision)"))
  (bind _returnvalue_x (`KismetMathLibrary.BreakVector2D` (`|GetInputActionValue`)))
  (return _returnvalue_x (`self.GetInputAxisKeyValue`) (`self.GetInputAxisKeyValue`)))

(fn `UserConstructionScript`)