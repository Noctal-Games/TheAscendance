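; BP_WillOWisp is a will-o'-wisp actor that bobs in place and notifies actors entering or leaving its range.
; Two chained timelines, one forward and one reversed, loop endlessly to drive the Wisp component's relative location.
; Mesh overlaps send in-range and out-of-range messages, passing the wisp itself, to actors implementing BPI_Wisp.
; GetPatrolRoute exposes its WispRoute, while its own InRange and OutRange functions are empty.
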(event `self.ReceiveBeginPlay`
  (bind (_direction _z_axis_movement) (`Timeline|Float` :!label _label)
    (:`Update`
      (`SceneComponent.K2_SetRelativeLocation` (`self.Wisp`) _z_axis_movement false false))
    (:`Finished`
      (bind (_direction_2 _z_axis_movement_2) (`Timeline|Timeline` :!via `ReverseFromEnd`)
        (:`Update`
          (`SceneComponent.K2_SetRelativeLocation` (`self.Wisp`) _z_axis_movement_2 false false))
        (:`Finished`
          (goto _label :!via `PlayFromStart`))))))

(event `self.Mesh.OnComponentBeginOverlap`
  (params (OverlappedComponent :type "PrimitiveComponent Object Reference") (OtherActor :type "Actor Object Reference") (OtherComp :type "PrimitiveComponent Object Reference") (OtherBodyIndex :type Integer) (bFromSweep :type Boolean) (SweepResult :type "HitResult Structure (by ref)"))
  (if (`KismetSystemLibrary.DoesImplementInterface` OtherActor "/Game/Developer/BenS/Interfaces/BPI_Wisp.BPI_Wisp_C")
    (message `/Game/Developer/BenS/Interfaces/BPI_Wisp.InRange` OtherActor self)))

(event `self.Mesh.OnComponentEndOverlap`
  (params (OverlappedComponent :type "PrimitiveComponent Object Reference") (OtherActor :type "Actor Object Reference") (OtherComp :type "PrimitiveComponent Object Reference") (OtherBodyIndex :type Integer))
  (if (`KismetSystemLibrary.DoesImplementInterface` OtherActor "/Game/Developer/BenS/Interfaces/BPI_Wisp.BPI_Wisp_C")
    (message `/Game/Developer/BenS/Interfaces/BPI_Wisp.OutRange` OtherActor self)))

(fn `GetPatrolRoute`
  (returns (WispRoute :type "/Game/Developer/BenS/Actors/WilloWisp/BP_SplineActor Object Reference"))
  (return (`self.WispRoute`)))

(fn `InRange`
  (params (Wisp :type "/Game/Developer/BenS/Actors/WilloWisp/BP_WillOWisp Object Reference")))

(fn `OutRange`
  (params (Wisp :type "/Game/Developer/BenS/Actors/WilloWisp/BP_WillOWisp Object Reference")))

(fn `UserConstructionScript`)