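; A one-shot player-interactable light switch that turns on its linked LightSource in the Will-o'-Wisp setup.
; BeginPlay binds Interact to OnInteract, and a DoOnce lets only the first interaction take effect.
; If the source holds a valid Wisp, it lights the source, then after a short delay sets that Wisp's walk speed.
; Otherwise it disables the source's collision before lighting it.
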(event `self.ReceiveBeginPlay`
  (add `BaseInteractableActor.OnInteract` (delegate `Interact`)))

(event `Interact`
  (bind _lightsource (`self.LightSource`))
  (bind _wisp (`/Game/Developer/BenS/Actors/WilloWisp/Interactables/Player/BP_LightSource.Wisp` _lightsource))
  (`/Engine/EditorBlueprintResources/StandardMacros.DoOnce` false
    (:`Completed`
      (`/Engine/EditorBlueprintResources/StandardMacros.IsValid` _wisp
        (:`Is Valid`
          (`/Game/Developer/BenS/Actors/WilloWisp/Interactables/Player/BP_LightSource.Light` _lightsource)
          (`KismetSystemLibrary.Delay` 0.5)
          (set `CharacterMovementComponent.MaxWalkSpeed` 200.0 (`Character.CharacterMovement` _wisp)))
        (:`Is Not Valid`
          (`PrimitiveComponent.SetCollisionProfileName` (`/Game/Developer/BenS/Actors/WilloWisp/Interactables/Player/BP_LightSource.Collision` _lightsource) "NoCollision" true)
          (`/Game/Developer/BenS/Actors/WilloWisp/Interactables/Player/BP_LightSource.Light` _lightsource))))))

(fn `GetPatrolRoute`
  (returns (WispRoute :type "/Game/Developer/BenS/Actors/WilloWisp/BP_SplineActor Object Reference"))
  (return null))

(fn `UserConstructionScript`
  (`parent.UserConstructionScript`))