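; BP_LightSource is an interactable light source for the WilloWisp actors.
; InRange stores the passed Wisp and, after a short delay, sets its max walk speed to zero.
; Light brightens the point light, starts the rotating movement and bobs the static mesh using two timelines, one played forward and one reversed, that trigger each other.
; GetPatrolRoute is an empty stub.
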(event `/Game/Developer/BenS/Interfaces/BPI_Wisp.InRange`
  (params (Wisp :type "/Game/Developer/BenS/Actors/WilloWisp/BP_WillOWisp Object Reference"))
  (bind _output_get (set `self.Wisp` Wisp))
  (`KismetSystemLibrary.Delay` 0.5)
  (set `CharacterMovementComponent.MaxWalkSpeed` 0.0 (`Character.CharacterMovement` _output_get)))

(event `Light`
  (`LightComponent.SetIntensity` (`self.PointLight`) 1000.0)
  (set `RotatingMovementComponent.RotationRate` (struct :`Yaw` 50.0) (`self.RotatingMovement`))
  (bind (_direction _z_axis_movement) (`Timeline|Timeline` :!label _label)
    (:`Update`
      (`SceneComponent.K2_SetRelativeLocation` (`self.StaticMesh`) _z_axis_movement false false))
    (:`Finished`
      (bind (_direction_2 _z_axis_movement_2) (`Timeline|Timeline_0` :!via `ReverseFromEnd`)
        (:`Update`
          (`SceneComponent.K2_SetRelativeLocation` (`self.StaticMesh`) _z_axis_movement_2 false false))
        (:`Finished`
          (goto _label :!via `PlayFromStart`))))))

(fn `GetPatrolRoute`
  (returns (WispRoute :type "/Game/Developer/BenS/Actors/WilloWisp/BP_SplineActor Object Reference"))
  (return null))

(fn `UserConstructionScript`
  (`parent.UserConstructionScript`))