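; BP_WispLever is a wisp interactable that opens a linked door when a Wisp comes in range.
; InRange runs a timed sequence with short delays: it halts the Wisp by zeroing its walk speed, calls DoorOpen on LinkedDoor, then sets a fixed walk speed again.
; The construction script defers to the parent, and GetPatrolRoute is an empty stub.
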(event `/Game/Developer/BenS/Interfaces/BPI_Wisp.InRange`
  (params (Wisp :type "/Game/Developer/BenS/Actors/WilloWisp/BP_WillOWisp Object Reference"))
  (bind _charactermovement (`Character.CharacterMovement` Wisp))
  (`KismetSystemLibrary.Delay` 0.5)
  (set `CharacterMovementComponent.MaxWalkSpeed` 0.0 _charactermovement)
  (`KismetSystemLibrary.Delay` 0.5)
  (`/Game/Developer/BenS/Actors/WilloWisp/Interactables/Wisp/BP_WispDoor.DoorOpen` (`self.LinkedDoor`))
  (`KismetSystemLibrary.Delay` 0.5)
  (set `CharacterMovementComponent.MaxWalkSpeed` 200.0 _charactermovement))

(fn `GetPatrolRoute`
  (returns (WispRoute :type "/Game/Developer/BenS/Actors/WilloWisp/BP_SplineActor Object Reference"))
  (return null))

(fn `UserConstructionScript`
  (`parent.UserConstructionScript`))