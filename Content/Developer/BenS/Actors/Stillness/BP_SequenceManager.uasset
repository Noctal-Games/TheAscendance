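; Manager for a fire-themed order puzzle in which BP_Sequence actors must be triggered in the correct sequence.
; CheckSequence compares each input index to CorrectSequence, advancing on a match and resetting on a mistake.
; Reset restores every BP_Sequence actor's fire effect, collision and interaction flag.
; Completion switches all their Niagara effects to slow fire and calls RestoreVision on every BP_SequenceSpawner.
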(event `self.ReceiveBeginPlay`
  (bind _returnvalue (`GameplayStatics.GetActorOfClass` "/Game/Developer/BenS/Actors/Stillness/BP_Sequence.BP_Sequence_C"))
  (set `self.Sequences` _returnvalue))

(fn `CheckSequence`
  (params (InputIndex :type Integer))
  (returns (`Return Value` :type Boolean))
  (if (== InputIndex (`|GetArrayItem` (`self.CorrectSequence`) (`self.CurrentStep`)))
    (bind _result (`/Engine/EditorBlueprintResources/StandardMacros.IncrementInt` (`self.CurrentStep`))
      (:`  `
        (if (== _result (`KismetArrayLibrary.Array_Length` (`self.CorrectSequence`)))
          (`self.PuzzleComplete`)
          (else
            (return true)))))
    (else
      (`self.ResetSequence`)
      (return false))))

(fn `PuzzleComplete`
  (`KismetSystemLibrary.PrintString` "Puzzle Complete")
  (`|ExecutionSequence`
    (:`then_0`
      (bind _outactors (`GameplayStatics.GetAllActorsOfClass` "/Game/Developer/BenS/Actors/Stillness/BP_Sequence.BP_Sequence_C"))
      (for _array_element _outactors
        (`NiagaraComponent.SetAsset` (`/Game/Developer/BenS/Actors/Stillness/BP_Sequence.Niagara` _array_element) "/Game/Developer/BenK/VFX_Tests/Stylised_Fire/Stylised_FireSLOW.Stylised_FireSLOW" true)))
    (:`then_1`
      (bind _outactors_2 (`GameplayStatics.GetAllActorsOfClass` "/Game/Developer/BenS/Actors/Stillness/BP_SequenceSpawner.BP_SequenceSpawner_C"))
      (for _array_element_2 _outactors_2
        (`/Game/Developer/BenS/Actors/Stillness/BP_SequenceSpawner.Restore Vision` _array_element_2)))))

(fn `ResetSequence`
  (set `self.CurrentStep` 0)
  (`KismetSystemLibrary.PrintString` "Reset")
  (bind _outactors (`GameplayStatics.GetAllActorsOfClass` "/Game/Developer/BenS/Actors/Stillness/BP_Sequence.BP_Sequence_C"))
  (for _array_element _outactors
    (`NiagaraComponent.SetAsset` (`/Game/Developer/BenS/Actors/Stillness/BP_Sequence.Niagara` _array_element) "/Game/Developer/BenK/VFX_Tests/Stylised_Fire/Stylised_Fire.Stylised_Fire" true)
    (`PrimitiveComponent.SetCollisionEnabled` (`/Game/Developer/BenS/Actors/Stillness/BP_Sequence.Sphere` _array_element) "QueryAndPhysics")
    (set `/Game/Developer/BenS/Actors/Stillness/BP_Sequence.HasBeenInteractedWith` false _array_element)))

(fn `UserConstructionScript`)