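; BP_Sequence is an interactable element of a sequence puzzle that lights a stylised fire effect when the sequence check passes.
; It finds the level's BP_SequenceManager on BeginPlay and passes its Sequence value to CheckSequence on first interaction.
; A passing check swaps the Niagara asset to the fire effect.
; A one-shot flag blocks further checks, and any later interaction disables the Sphere's collision.
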(event `self.ReceiveBeginPlay`
  (bind _returnvalue (`GameplayStatics.GetActorOfClass` "/Game/Developer/BenS/Actors/Stillness/BP_SequenceManager.BP_SequenceManager_C"))
  (set `self.SequenceManager` _returnvalue))

(event `/Game/Developer/BenS/Interfaces/BPI_PlayerInteract.OnInteract`
  (if (`self.HasBeenInteractedWith`)
    (`PrimitiveComponent.SetCollisionEnabled` (`self.Sphere`) "NoCollision")
    (else
      (set `self.HasBeenInteractedWith` true)
      (bind _return_value (`/Game/Developer/BenS/Actors/Stillness/BP_SequenceManager.CheckSequence` (`self.SequenceManager`) (`self.Sequence`)))
      (if _return_value
        (`NiagaraComponent.SetAsset` (`self.Niagara`) "/Game/Developer/BenK/VFX_Tests/Stylised_Fire/Stylised_FireINST1.Stylised_FireINST1" true)))))

(fn `UserConstructionScript`)