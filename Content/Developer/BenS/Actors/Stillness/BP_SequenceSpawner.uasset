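; Trigger actor that starts a Fear Trial encounter when the player overlaps its collision volume.
; It lights the level's red wall torches one by one through a delayed recursive event.
; After a short delay, it once fades the height fog to a set density with black albedo via a reversible timeline.
; It then spawns four numbered BP_Sequence actors and creates a boss through the game mode.
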(event `self.ReceiveBeginPlay`
  (`|ExecutionSequence`
    (:`then_0`
      (bind _outactors (`GameplayStatics.GetAllActorsOfClass` "/Script/Engine.ExponentialHeightFog"))
      (set `self.Fog` (`|GetArrayItem` _outactors)))
    (:`then_1`
      (set `self.IncrementID` 0)
      (bind _outactors_2 (`GameplayStatics.GetAllActorsOfClass` "/Game/Developer/BenS/Actors/Stillness/BP_WallTorch_FearTrial.BP_WallTorch_FearTrial_C"))
      (set `self.Torches` _outactors_2))))

(event `self.Collision.OnComponentBeginOverlap`
  (params (OverlappedComponent :type "PrimitiveComponent Object Reference") (OtherActor :type "Actor Object Reference") (OtherComp :type "PrimitiveComponent Object Reference") (OtherBodyIndex :type Integer) (bFromSweep :type Boolean) (SweepResult :type "HitResult Structure (by ref)"))
  (cast `/Game/Developer/BenS/Characters/Blueprints/BP_PlayerTestGuy` OtherActor)
  (`|ExecutionSequence`
    (:`then_0`
      (`self.TurnOnTorches`))
    (:`then_1`
      (`KismetSystemLibrary.Delay` 3.0)
      (`/Engine/EditorBlueprintResources/StandardMacros.DoOnce` false
        (:`Completed`
          (`self.ReduceVision`)
          (`self.SpawnSequenceActors`)
          (`KismetSystemLibrary.Delay` 1.0)
          (set `self.Boss` (`PlayableGameMode.CreateEnemyFromID` (`CoreFunctionLibrary.GetPlayableGameMode`) 10)))))))

(event `ReduceVision`
  (bind (_direction _fogfadespeed) (`Timeline|FogFadeTimeline` :!label _label)
    (:`Update`
      (`ExponentialHeightFogComponent.SetFogDensity` (`ExponentialHeightFog.Component` (`self.Fog`)) (`KismetMathLibrary.Lerp` (`self.DefaultFogDensity`) (`self.FogDensity`) _fogfadespeed))
      (`ExponentialHeightFogComponent.SetVolumetricFogAlbedo` (`ExponentialHeightFog.Component` (`self.Fog`)) (make `Color` 0 0 0 255)))))

(event `Restore Vision`
  (goto _label :!via `Reverse`))

(event `TurnOnTorches`
  (if (< (`self.IncrementID`) (`KismetArrayLibrary.Array_Length` (`self.Torches`)))
    (`SceneComponent.SetVisibility` (`/Game/Developer/BenS/Actors/Stillness/BP_WallTorch_FearTrial.P_Fire_WallTorch_RED` (`|GetArrayItem` (`self.Torches`) (`self.IncrementID`))) true false)
    (`SceneComponent.SetVisibility` (`/Game/Developer/BenS/Actors/Stillness/BP_WallTorch_FearTrial.PointLight` (`|GetArrayItem` (`self.Torches`) (`self.IncrementID`))) true false)
    (`/Engine/EditorBlueprintResources/StandardMacros.IncrementInt` (`self.IncrementID`)
      (:`  `
        (`KismetSystemLibrary.Delay` 0.05)
        (`self.TurnOnTorches`)))))

(fn `SpawnSequenceActors`
  (bind _returnvalue (`|SpawnActorFromClass` "/Game/Developer/BenS/Actors/Stillness/BP_Sequence.BP_Sequence_C" (`KismetMathLibrary.MakeTransform` (`self.Sequence_01`)) "Undefined" "MultiplyWithRoot" null null))
  (set `/Game/Developer/BenS/Actors/Stillness/BP_Sequence.Sequence` 1 _returnvalue)
  (bind _returnvalue_2 (`|SpawnActorFromClass` "/Game/Developer/BenS/Actors/Stillness/BP_Sequence.BP_Sequence_C" (`KismetMathLibrary.MakeTransform` (`self.Sequence_02`)) "Undefined" "MultiplyWithRoot" null null))
  (set `/Game/Developer/BenS/Actors/Stillness/BP_Sequence.Sequence` 2 _returnvalue_2)
  (bind _returnvalue_3 (`|SpawnActorFromClass` "/Game/Developer/BenS/Actors/Stillness/BP_Sequence.BP_Sequence_C" (`KismetMathLibrary.MakeTransform` (`self.Sequence_03`)) "Undefined" "MultiplyWithRoot" null null))
  (set `/Game/Developer/BenS/Actors/Stillness/BP_Sequence.Sequence` 3 _returnvalue_3)
  (bind _returnvalue_4 (`|SpawnActorFromClass` "/Game/Developer/BenS/Actors/Stillness/BP_Sequence.BP_Sequence_C" (`KismetMathLibrary.MakeTransform` (`self.Sequence_04`)) "Undefined" "MultiplyWithRoot" null null))
  (set `/Game/Developer/BenS/Actors/Stillness/BP_Sequence.Sequence` 4 _returnvalue_4))

(fn `UserConstructionScript`)