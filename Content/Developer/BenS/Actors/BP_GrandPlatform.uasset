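; BP_GrandPlatform is an actor whose four stacked platform meshes rise to successively lower heights in a staggered sequence.
; Timeline_1 plays on BeginPlay and on the first BP_PlayerTestGuy overlap with the Sphere.
; Each timeline lerps one mesh's relative Z and starts the next through a one-second Delay on its Update, so the movements can overlap.
; The last timeline zeroes RotatingMovement's rotation rate when it finishes.
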(event `self.ReceiveBeginPlay`
  (bind (_direction _alpha) (`Timeline|Timeline_1` :!label _label)
    (:`Update`
      (`SceneComponent.K2_SetRelativeLocation` (`self.BB_1stPlatform_StaticMesh`) (`KismetMathLibrary.MakeVector` 0.0 0.0 (`KismetMathLibrary.Lerp` 0.0 1679.8 _alpha)) false false)
      (`KismetSystemLibrary.Delay` 1.0)
      (bind (_direction_2 _alpha_2) (`Timeline|Timeline_2`)
        (:`Update`
          (`SceneComponent.K2_SetRelativeLocation` (`self.BB_1stPlatform2_StaticMesh`) (`KismetMathLibrary.MakeVector` 0.0 0.0 (`KismetMathLibrary.Lerp` 0.0 1271.7 _alpha_2)) false false)
          (`KismetSystemLibrary.Delay` 1.0)
          (bind (_direction_3 _alpha_3) (`Timeline|Timeline_3`)
            (:`Update`
              (`SceneComponent.K2_SetRelativeLocation` (`self.BB_1stPlatform3_StaticMesh`) (`KismetMathLibrary.MakeVector` 0.0 0.0 (`KismetMathLibrary.Lerp` 0.0 737.5 _alpha_3)) false false)
              (`KismetSystemLibrary.Delay` 1.0)
              (bind (_direction_4 _alpha_4) (`Timeline|Timeline_4`)
                (:`Update`
                  (`SceneComponent.K2_SetRelativeLocation` (`self.BB_1stPlatform4_StaticMesh`) (`KismetMathLibrary.MakeVector` 0.0 0.0 (`KismetMathLibrary.Lerp` 0.0 190.5 _alpha_4)) false false))
                (:`Finished`
                  (set `RotatingMovementComponent.RotationRate` (struct) (`self.RotatingMovement`)))))))))))

(event `self.Sphere.OnComponentBeginOverlap`
  (params (OverlappedComponent :type "PrimitiveComponent Object Reference") (OtherActor :type "Actor Object Reference") (OtherComp :type "PrimitiveComponent Object Reference") (OtherBodyIndex :type Integer) (bFromSweep :type Boolean) (SweepResult :type "HitResult Structure (by ref)"))
  (cast `/Game/Developer/BenS/Characters/Blueprints/BP_PlayerTestGuy` OtherActor)
  (`/Engine/EditorBlueprintResources/StandardMacros.DoOnce` false
    (:`Completed`
      (goto _label))))

(fn `UserConstructionScript`)