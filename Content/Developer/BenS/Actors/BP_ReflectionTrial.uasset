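; Trigger actor that runs a three-phase Trial of Reflection boss encounter, started once when BP_PlayerTestGuy overlaps its collision.
; Tick polls enemy health: the first reflection is removed at a health threshold, replaced by Melee, Tank and Mage enemies with trial materials.
; Once all three die, tallied in TempArray, a Corrupted Reflection spawns.
; Its death prints completion and destroys the actor after a delay.
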(event `self.collision.OnComponentBeginOverlap`
  (params (OverlappedComponent :type "PrimitiveComponent Object Reference") (OtherActor :type "Actor Object Reference") (OtherComp :type "PrimitiveComponent Object Reference") (OtherBodyIndex :type Integer) (bFromSweep :type Boolean) (SweepResult :type "HitResult Structure (by ref)"))
  (cast `/Game/Developer/BenS/Characters/Blueprints/BP_PlayerTestGuy` OtherActor)
  (`/Engine/EditorBlueprintResources/StandardMacros.DoOnce` false
    (:`Completed`
      (bind _returnvalue (`PlayableGameMode.CreateEnemyFromID` (`CoreFunctionLibrary.GetPlayableGameMode`) 2))
      (set `self.ReflectionOne` _returnvalue))))

(event `self.ReceiveTick`
  (params (DeltaSeconds :type "Float (single-precision)"))
  (bind _returnvalue (`CoreFunctionLibrary.GetPlayableGameMode`))
  (`|ExecutionSequence`
    (:`then_0`
      (bind _reflectionone (`self.ReflectionOne`)
        (:`then`
          (bind _returnvalue_2 (`Susceptible.GetStat` _reflectionone "HEALTH"))
          (if (<= _returnvalue_2 70)
            (`self.K2_DestroyActor` (`self.ReflectionOne`))
            (`/Engine/EditorBlueprintResources/StandardMacros.DoOnce` false
              (:`Completed`
                (`|ExecutionSequence`
                  (:`then_0`
                    (bind _returnvalue_3 (`PlayableGameMode.CreateEnemyFromID` _returnvalue 3))
                    (bind _output_get (set `self.Melee` _returnvalue_3))
                    (for (_ _array_index) (`self.MaterialIndex`)
                      (`PrimitiveComponent.SetMaterial` (`Character.Mesh` _output_get) _array_index "/Game/Developer/Courtney/Enemies/TrialOfReflectionShadows/M_TrialOfReflection_Beast.M_TrialOfReflection_Beast")
                      (`SceneComponent.K2_SetWorldLocation` (`Character.CapsuleComponent` _output_get) (0.0 0.0 0.0) false false)))
                  (:`then_1`
                    (bind _returnvalue_4 (`PlayableGameMode.CreateEnemyFromID` _returnvalue 4))
                    (bind _output_get_2 (set `self.tank` _returnvalue_4))
                    (for (_ _array_index_2) (`self.MaterialIndex`)
                      (`PrimitiveComponent.SetMaterial` (`Character.Mesh` _output_get_2) _array_index_2 "/Game/Developer/Courtney/Enemies/TrialOfReflectionShadows/M_TrialOfReflection_Guardian.M_TrialOfReflection_Guardian")
                      (`SceneComponent.K2_SetWorldLocation` (`Character.CapsuleComponent` _output_get_2) (0.0 0.0 0.0) false false)))
                  (:`then_2`
                    (bind _returnvalue_5 (`PlayableGameMode.CreateEnemyFromID` _returnvalue 5))
                    (bind _output_get_3 (set `self.mage` _returnvalue_5))
                    (for (_ _array_index_3) (`self.MaterialIndex`)
                      (`PrimitiveComponent.SetMaterial` (`Character.Mesh` _output_get_3) _array_index_3 "/Game/Developer/Courtney/Enemies/TrialOfReflectionShadows/M_TrialOfReflection_Ascendant.M_TrialOfReflection_Ascendant")
                      (`SceneComponent.K2_SetWorldLocation` (`Character.CapsuleComponent` _output_get_3) (0.0 0.0 0.0) false false))))))))
        (:`else`)))
    (:`then_1`
      (bind _melee (`self.Melee`)
        (:`then`
          (bind _returnvalue_6 (`Susceptible.GetStat` _melee "HEALTH"))
          (if (<= _returnvalue_6 0)
            (`/Engine/EditorBlueprintResources/StandardMacros.DoOnce` false
              (:`Completed`
                (`KismetArrayLibrary.Array_Add` (`self.TempArray`) 1)
                (`self.K2_DestroyActor` (`self.Melee`))))))
        (:`else`)))
    (:`then_2`
      (bind _tank (`self.tank`)
        (:`then`
          (bind _returnvalue_7 (`Susceptible.GetStat` _tank "HEALTH"))
          (if (<= _returnvalue_7 0)
            (`/Engine/EditorBlueprintResources/StandardMacros.DoOnce` false
              (:`Completed`
                (`KismetArrayLibrary.Array_Add` (`self.TempArray`) 2)
                (`self.K2_DestroyActor` (`self.tank`))))))
        (:`else`)))
    (:`then_3`
      (bind _mage (`self.mage`)
        (:`then`
          (bind _returnvalue_8 (`Susceptible.GetStat` _mage "HEALTH"))
          (if (<= _returnvalue_8 0)
            (`/Engine/EditorBlueprintResources/StandardMacros.DoOnce` false
              (:`Completed`
                (`KismetArrayLibrary.Array_Add` (`self.TempArray`) 3)
                (`self.K2_DestroyActor` (`self.mage`))))))
        (:`else`)))
    (:`then_4`
      (if (>= (`KismetArrayLibrary.Array_Length` (`self.TempArray`)) 3)
        (`/Engine/EditorBlueprintResources/StandardMacros.DoOnce` false
          (:`Completed`
            (bind _returnvalue_9 (`PlayableGameMode.CreateEnemyFromID` (`CoreFunctionLibrary.GetPlayableGameMode`) 6))
            (bind _output_get_4 (set `self.CorruptedReflection` _returnvalue_9))
            (for (_ _array_index_4) (`self.MaterialIndex`)
              (`PrimitiveComponent.SetMaterial` (`Character.Mesh` _output_get_4) _array_index_4 "/Game/Developer/Courtney/Enemies/TrialOfReflectionShadows/M_TrialOfReflection_ShadowPhase3.M_TrialOfReflection_ShadowPhase3")
              (`SceneComponent.K2_SetWorldLocation` (`Character.CapsuleComponent` _output_get_4) (0.0 0.0 0.0) false false))))))
    (:`then_5`
      (bind _corruptedreflection (`self.CorruptedReflection`)
        (:`then`
          (bind _returnvalue_10 (`Susceptible.GetStat` _corruptedreflection "HEALTH"))
          (if (<= _returnvalue_10 0)
            (`/Engine/EditorBlueprintResources/StandardMacros.DoOnce` false
              (:`Completed`
                (`self.K2_DestroyActor` (`self.CorruptedReflection`))
                (`KismetSystemLibrary.PrintString` "Trial 1 complete")
                (`KismetSystemLibrary.Delay` 3.0)
                (`self.K2_DestroyActor`)))))
        (:`else`)))))

(fn `UserConstructionScript`)