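; Item inspection actor that displays an examined item's mesh alongside a W_Inspect widget carrying its name, description and riddle data.
; Inspect swaps the mesh, opens the widget and switches to UI-only input with a cursor; separate events set starting rotation and scale.
; Left-drag rotates the mesh, the wheel zooms via clamped SceneCapture FOV, and right-click resets both, though a comment marks input as temporarily disabled.
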(event `SetInspectRotation`
  (params (ItemRotation :type "Rotator Structure"))
  (bind _staticmesh (`self.StaticMesh`))
  (bind (_returnvalue_location _returnvalue_rotation _returnvalue_scale) (`KismetMathLibrary.BreakTransform` (`SceneComponent.K2_GetComponentToWorld` _staticmesh)))
  (bind _output_get (set `self.ItemInitialRotation` ItemRotation))
  (`SceneComponent.K2_SetWorldTransform` _staticmesh (`KismetMathLibrary.MakeTransform` _returnvalue_location _output_get _returnvalue_scale) false false))

(event `SetInspectScale`
  (params (InspectScale :type "Vector Structure"))
  (bind _staticmesh (`self.StaticMesh`))
  (bind (_returnvalue_location _returnvalue_rotation) (`KismetMathLibrary.BreakTransform` (`SceneComponent.K2_GetComponentToWorld` _staticmesh)))
  (`SceneComponent.K2_SetWorldTransform` _staticmesh (`KismetMathLibrary.MakeTransform` _returnvalue_location _returnvalue_rotation InspectScale) false false))

(event `/Game/Developer/BenS/Interfaces/BPI_Player_Functions.Inspect`
  (params (Character :type "/Game/Developer/BenS/Characters/Blueprints/BP_PlayerTestGuy Object Reference") (InspectedItem :type "StaticMesh Object Reference") (`Item Name` :type Text) (`Item Description` :type Text) (ID :type Integer) (Actor :type "/Game/Developer/BenS/Actors/Dilligance/BP_RiddleItem Object Reference"))
  (bind _returnvalue (`GameplayStatics.GetPlayerController` 0))
  (set `self.Character` Character)
  (`StaticMeshComponent.SetStaticMesh` (`self.StaticMesh`) InspectedItem)
  (bind _returnvalue_2 (`|CreateWidget` "/Game/Developer/BenS/Actors/Dilligance/UI/Inspect/W_Inspect.W_Inspect_C" null `Item Name` `Item Description` (make `/Game/Developer/BenS/Actors/Dilligance/S_Riddle` ID InspectedItem) Actor))
  (bind _output_get (set `self.InspectWidget` _returnvalue_2))
  (`UserWidget.AddToViewport` _output_get 0)
  (`WidgetBlueprintLibrary.SetInputMode_UIOnlyEx` _returnvalue null)
  (set `PlayerController.bShowMouseCursor` true _returnvalue))

(event `Key|RightMouseButton` :paused true
  (params (Key :type "Key Structure"))
  ;[0.7031 0 0 0.4783] Temp disabled until i fix the input
  (:`Pressed`
    (`SceneComponent.K2_SetWorldRotation` (`self.StaticMesh`) (`self.ItemInitialRotation`) false false)
    (set `SceneCaptureComponent2D.FOVAngle` 50.0 (`self.SceneCaptureComponent2D`))))

(event `InputAxisKey|MouseX` :paused true
  (params (AxisValue :type "Float (single-precision)"))
  ;[0.7031 0 0 0.4783] Temp disabled until i fix the input
  (if (`self.Rotate?`)
    (`SceneComponent.K2_SetWorldRotation` (`self.StaticMesh`) (`KismetMathLibrary.ComposeRotators` (`SceneComponent.K2_GetComponentRotation` (`self.StaticMesh`)) (`KismetMathLibrary.MakeRotator` 0.0 0.0 (* AxisValue -3.0))) false false)))

(event `Key|LeftMouseButton` :paused true
  (params (Key :type "Key Structure"))
  ;[0.7031 0 0 0.4783] Temp disabled until i fix the input
  (:`Pressed`
    (set `self.Rotate?` true))
  (:`Released`
    (set `self.Rotate?` false)))

(event `InputAxisKey|MouseY` :paused true
  (params (AxisValue :type "Float (single-precision)"))
  ;[0.7031 0 0 0.4783] Temp disabled until i fix the input
  (if (`self.Rotate?`)
    (`SceneComponent.K2_SetWorldRotation` (`self.StaticMesh`) (`KismetMathLibrary.ComposeRotators` (`SceneComponent.K2_GetComponentRotation` (`self.StaticMesh`)) (`KismetMathLibrary.MakeRotator` 0.0 (* AxisValue -3.0))) false false)))

(event `Key|MouseScrollUp` :paused true
  (params (Key :type "Key Structure"))
  (bind _scenecapturecomponent2d (`self.SceneCaptureComponent2D`))
  ;[0.7031 0 0 0.4783] Temp disabled until i fix the input
  (:`Pressed`
    (set `SceneCaptureComponent2D.FOVAngle` (`KismetMathLibrary.FClamp` (- (`SceneCaptureComponent2D.FOVAngle` _scenecapturecomponent2d) 1.0) 30.0 80.0) _scenecapturecomponent2d)))

(event `Key|MouseScrollDown` :paused true
  (params (Key :type "Key Structure"))
  (bind _scenecapturecomponent2d (`self.SceneCaptureComponent2D`))
  ;[0.7031 0 0 0.4783] Temp disabled until i fix the input
  (:`Pressed`
    (set `SceneCaptureComponent2D.FOVAngle` (`KismetMathLibrary.FClamp` (+ (`SceneCaptureComponent2D.FOVAngle` _scenecapturecomponent2d) 1.0) 30.0 80.0) _scenecapturecomponent2d)))

(fn `GetPatrolRoute`
  (returns (WispRoute :type "/Game/Developer/BenS/Actors/WilloWisp/BP_SplineActor Object Reference"))
  (return null))

(fn `UserConstructionScript`
  (`parent.UserConstructionScript`))