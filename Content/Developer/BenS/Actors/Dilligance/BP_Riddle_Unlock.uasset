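; Riddle unlock interactable that opens a seamless portal when the player brings the correct pair of items.
; On interact, it spawns a collision-free display copy of each item in the player's riddle data and gathers their unique IDs.
; When exactly two IDs match the required pair, it spawns a linked portal, clears both lists and ignores Visibility traces.
; A wrong pair only prints a failure message.
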(event `self.ReceiveBeginPlay`
  (add `BaseInteractableActor.OnInteract` (delegate `Interact`)))

(event `Interact`
  (for _array_element (`/Game/Developer/BenS/Characters/Blueprints/BP_PlayerTestGuy.RiddleItemData` (cast `/Game/Developer/BenS/Characters/Blueprints/BP_PlayerTestGuy` (`GameplayStatics.GetPlayerCharacter` 0) :!pure true))
    (bind (_itemid _inspecteditem) (break `/Game/Developer/BenS/Actors/Dilligance/S_Riddle` _array_element))
    (bind _returnvalue (`|SpawnActorFromClass` "/Game/Developer/BenS/Actors/Dilligance/BP_RiddleItem.BP_RiddleItem_C" (`KismetMathLibrary.MakeTransform` (`SceneComponent.K2_GetComponentLocation` (`self.Scene`))) "Undefined" "MultiplyWithRoot" null _itemid _inspecteditem null))
    (`PrimitiveComponent.SetCollisionProfileName` (`/Game/Developer/BenH/Test/BP_TestInteractableActor.StaticMesh` _returnvalue) "NoCollision" true)
    (`KismetArrayLibrary.Array_AddUnique` (`self.Collected IDs`) (`/Game/Developer/BenS/Actors/Dilligance/BP_RiddleItem.ID` _returnvalue))
    (`self.CheckPuzzleItem`)))

(event `Success`
  (`|SpawnActorFromClass` "/Game/Developer/BenS/Portal/BP_SeamlessPortal.BP_SeamlessPortal_C" (`KismetMathLibrary.MakeTransform` (`self.PortalLocation`) (`self.PortalRotation`)) "Undefined" "MultiplyWithRoot" null (`self.LinkedPortal`) null)
  (`KismetArrayLibrary.Array_Clear` (`self.Collected IDs`))
  (`KismetArrayLibrary.Array_Clear` (`/Game/Developer/BenS/Characters/Blueprints/BP_PlayerTestGuy.RiddleItemData` (cast `/Game/Developer/BenS/Characters/Blueprints/BP_PlayerTestGuy` (`GameplayStatics.GetPlayerCharacter` 0) :!pure true))))

(event `Failure`
  (`KismetSystemLibrary.PrintString` "fail"))

(fn `CheckPuzzleItem`
  (bind _collected_ids (`self.Collected IDs`))
  (if (== (`KismetArrayLibrary.Array_Length` (`self.Collected IDs`)) 2)
    (if (and (`KismetArrayLibrary.Array_Contains` _collected_ids (`self.RequiredID1`)) (`KismetArrayLibrary.Array_Contains` _collected_ids (`self.RequiredID2`)))
      (`self.Success`)
      (`PrimitiveComponent.SetCollisionResponseToChannel` (`self.StaticMesh`) "ECC_Visibility" "ECR_Ignore")
      (else
        (`self.Failure`)))))

(fn `UserConstructionScript`
  (`parent.UserConstructionScript`))