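; Riddle item the player can pick up and carry, with configurable mesh, name and description.
; Interact alternates between grabbing the camera-trace hit component through the player's PhysicsHandle and releasing it, toggling Pawn/WorldDynamic collision and a lift Niagara effect.
; While held, Tick moves the handle target in front of the camera.
; Proximity overlap spawns a screen-space description widget, removed when the player leaves or while the item is held.
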(event `self.ReceiveBeginPlay`
  (bind _staticmesh (`self.StaticMesh`))
  (add `BaseInteractableActor.OnInteract` (delegate `Interact`))
  (set `self.ItemInitialLocation` (`SceneComponent.K2_GetComponentLocation` _staticmesh))
  (set `self.ItemInitialRotation` (`SceneComponent.K2_GetComponentRotation` _staticmesh))
  (bind _asbp_player_test_guy (cast `/Game/Developer/BenS/Characters/Blueprints/BP_PlayerTestGuy` (`GameplayStatics.GetPlayerCharacter` 0)))
  (set `self.Player` _asbp_player_test_guy))

(event `Interact`
  (`/Engine/EditorBlueprintResources/StandardMacros.FlipFlop`
    (:`A`
      (`self.GrabComponent`))
    (:`B`
      (`self.ReleaseComponent`))))

(event `self.ReceiveTick`
  (params (DeltaSeconds :type "Float (single-precision)"))
  (bind _player (`self.Player`))
  (bind _physicshandle (`/Game/Developer/BenS/Characters/Blueprints/BP_PlayerTestGuy.PhysicsHandle` _player))
  (if (`self.IsGrabbed`)
    (`PhysicsHandleComponent.SetTargetLocation` _physicshandle (`.End` (`self.LineTrace` 200.0)))
    (`PhysicsHandleComponent.SetTargetRotation` _physicshandle (`SceneComponent.K2_GetComponentRotation` (`PlayerCharacter.m_Camera` _player)))
    (`self.NotGrabbed`)))

(event `self.WidgetDetection.OnComponentBeginOverlap`
  (params (OverlappedComponent :type "PrimitiveComponent Object Reference") (OtherActor :type "Actor Object Reference") (OtherComp :type "PrimitiveComponent Object Reference") (OtherBodyIndex :type Integer) (bFromSweep :type Boolean) (SweepResult :type "HitResult Structure (by ref)"))
  (cast `/Game/Developer/BenS/Characters/Blueprints/BP_PlayerTestGuy` OtherActor)
  (if (not (`self.IsGrabbed`))
    (`self.WidgetInteraction`
      (:`then`)
      (:`else`
        (bind _returnvalue (`|CreateWidget` "/Game/Developer/BenS/Actors/Dilligance/UI/W_RiddleItemDescription.W_RiddleItemDescription_C" null (`self.ItemName`) (`self.ItemDescription`)))
        (bind _output_get (set `self.Widget` _returnvalue))
        (bind _returnvalue_2 (`AddComponent|NODE_AddWidgetComponent-0`))
        (bind _output_get_2 (set `self.WidgetInteraction` _returnvalue_2))
        (`WidgetComponent.SetWidget` _output_get_2 _output_get)
        (`WidgetComponent.SetWidgetSpace` _output_get_2 "Screen")
        (`WidgetComponent.SetDrawAtDesiredSize` _output_get_2 true)
        (`PrimitiveComponent.SetCollisionEnabled` _output_get_2 "NoCollision")
        (`SceneComponent.K2_AttachToComponent` _output_get_2 (`self.StaticMesh`) "None" "SnapToTarget" "SnapToTarget" "SnapToTarget" true)))))

(event `NotGrabbed`
  (bind _widgetinteraction (`self.WidgetInteraction` :!label _label)
    (:`then`
      (`ActorComponent.K2_DestroyComponent` _widgetinteraction))
    (:`else`)))

(event `self.WidgetDetection.OnComponentEndOverlap`
  (params (OverlappedComponent :type "PrimitiveComponent Object Reference") (OtherActor :type "Actor Object Reference") (OtherComp :type "PrimitiveComponent Object Reference") (OtherBodyIndex :type Integer))
  (cast `/Game/Developer/BenS/Characters/Blueprints/BP_PlayerTestGuy` OtherActor)
  (goto _label))

(fn `GrabComponent`
  (bind (_start _end) (`self.LineTrace` 500.0))
  (bind (_outhit _returnvalue) (`KismetSystemLibrary.LineTraceSingle` :`Start` _start :`End` _end :`TraceChannel` "TraceTypeQuery1" :`bIgnoreSelf` false))
  (if _returnvalue
    (bind _output_get (set `self.Hit Component` (`.HitComponent` (`GameplayStatics.BreakHitResult` _outhit))))
    (`PrimitiveComponent.SetSimulatePhysics` _output_get true)
    (`PrimitiveComponent.SetCollisionResponseToChannel` _output_get "ECC_Pawn" "ECR_Ignore")
    (`PrimitiveComponent.SetCollisionResponseToChannel` _output_get "ECC_WorldDynamic" "ECR_Ignore")
    (bind _asbp_player_test_guy (cast `/Game/Developer/BenS/Characters/Blueprints/BP_PlayerTestGuy` (`GameplayStatics.GetPlayerCharacter` 0)))
    (`PhysicsHandleComponent.GrabComponentAtLocationWithRotation` (`/Game/Developer/BenS/Characters/Blueprints/BP_PlayerTestGuy.PhysicsHandle` _asbp_player_test_guy) _output_get "None" (`SceneComponent.K2_GetComponentLocation` _output_get) (`SceneComponent.K2_GetComponentRotation` _output_get))
    (`NiagaraComponent.SetAsset` (`self.Niagara`) "/Game/Developer/BenS/Actors/Dilligance/NS_Lift.NS_Lift" true)
    (set `self.IsGrabbed` true)))

(fn `LineTrace`
  (params (Range :type "Float (double-precision)"))
  (returns (Start :type "Vector Structure") (End :type "Vector Structure"))
  (bind _m_camera (`PlayerCharacter.m_Camera` (`self.Player`)))
  (bind _returnvalue (`SceneComponent.K2_GetComponentLocation` _m_camera))
  (return _returnvalue (+ _returnvalue (* (`KismetMathLibrary.GetForwardVector` (`SceneComponent.K2_GetComponentRotation` _m_camera)) (`local.Range`)))))

(fn `ReleaseComponent`
  (bind _hit_component (`self.Hit Component`))
  (`PhysicsHandleComponent.ReleaseComponent` (`/Game/Developer/BenS/Characters/Blueprints/BP_PlayerTestGuy.PhysicsHandle` (`self.Player`)))
  (set `self.IsGrabbed` false)
  (`PrimitiveComponent.SetCollisionResponseToChannel` _hit_component "ECC_Pawn" "ECR_Block")
  (`PrimitiveComponent.SetCollisionResponseToChannel` _hit_component "ECC_WorldDynamic" "ECR_Block")
  (`NiagaraComponent.SetAsset` (`self.Niagara`) null true))

(fn `UserConstructionScript`
  (`StaticMeshComponent.SetStaticMesh` (`self.StaticMesh`) (`self.ItemMesh`)))