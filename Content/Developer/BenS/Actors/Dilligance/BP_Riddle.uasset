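; BP_Riddle is an interactable actor that presents a riddle UI to the player.
; On BeginPlay it binds to its OnInteract event, which creates and stores a W_Riddle widget, adds it to the viewport and switches the first player controller to UI-only input with the mouse cursor shown.
; GetPatrolRoute is an empty stub, and the construction script only calls the parent.
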(event `self.ReceiveBeginPlay`
  (add `BaseInteractableActor.OnInteract` (delegate `Interact`)))

(event `Interact`
  (bind _returnvalue (`GameplayStatics.GetPlayerController` 0))
  (bind _returnvalue_2 (`|CreateWidget` "/Game/Developer/BenS/Actors/Dilligance/UI/W_Riddle.W_Riddle_C"))
  (bind _output_get (set `self.Riddle` _returnvalue_2))
  (`WidgetBlueprintLibrary.SetInputMode_UIOnlyEx` _returnvalue _output_get)
  (`UserWidget.AddToViewport` _output_get 0)
  (set `PlayerController.bShowMouseCursor` true _returnvalue))

(fn `GetPatrolRoute`
  (returns (WispRoute :type "/Game/Developer/BenS/Actors/WilloWisp/BP_SplineActor Object Reference"))
  (return null))

(fn `UserConstructionScript`
  (`parent.UserConstructionScript`))