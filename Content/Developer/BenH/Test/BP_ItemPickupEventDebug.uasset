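; BP_ItemPickupEventDebug is a developer test actor that reports player item pickups through on-screen debug text.
; On BeginPlay it binds an event to the GameEventSubsystem's item pickup delegate.
; When that fires, a helper function prints the picked-up item's ID and amount with PrintString.
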(event `self.ReceiveBeginPlay`
  (add `GameEventSubsystem.OnItemPickupBP` (subsystem `GameEventSubsystem`) (delegate `OnItemPickupBP_Event`)))

(event `OnItemPickupBP_Event`
  (params (ID :type Integer) (Amount :type Integer))
  (`self.ItemPickupDebugMessage` ID Amount))

(fn `ItemPickupDebugMessage`
  (params (id :type Integer) (amount :type Integer))
  (`KismetSystemLibrary.PrintString` (`KismetStringLibrary.Concat_StrStr` (`KismetStringLibrary.Concat_StrStr` "Player picked up item: " (`KismetStringLibrary.Conv_IntToString` id)) (`KismetStringLibrary.Concat_StrStr` (`KismetStringLibrary.Concat_StrStr` "(" (`KismetStringLibrary.Conv_IntToString` amount)) ")"))))

(fn `UserConstructionScript`)