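; Developer test actor that assigns a spell loadout to the player character when play begins.
; After a short delay on BeginPlay, it gets the player character and checks that it is valid.
; It then passes its main and off spell variables, each with a primary and alt slot, as an array to the player's TestSetSpells function.
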(event `self.ReceiveBeginPlay`
  (`KismetSystemLibrary.Delay` 1.0)
  (bind _output_get (set `self.Player` (`CoreFunctionLibrary.GetPlayerCharacter`)))
  (if (`KismetSystemLibrary.IsValid` _output_get)
    (`PlayerCharacter.TestSetSpells` (`self.Player`) (`|MakeArray` (`self.MainPrimarySpell`) (`self.MainAltSpell`) (`self.OffPrimarySpell`) (`self.OffAltSpell`)))))

(fn `UserConstructionScript`)