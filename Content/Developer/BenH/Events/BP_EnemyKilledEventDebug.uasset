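; A debug actor that tests the game event subsystem's enemy-killed notification by printing messages to screen.
; On BeginPlay it binds a handler to the subsystem's OnEnemyKilledBP event.
; The handler passes the received Id to EnemyKilledDebugMessage, which prints a yellow kill message for one hardcoded Id and a red ignore message for any other.
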(event `self.ReceiveBeginPlay`
  (add `GameEventSubsystem.OnEnemyKilledBP` (subsystem `GameEventSubsystem`) (delegate `OnEnemyKilledBP_Event`)))

(event `OnEnemyKilledBP_Event`
  (params (id :type Integer))
  (`self.EnemyKilledDebugMessage` id))

(fn `EnemyKilledDebugMessage`
  (params (id :type Integer))
  (if (== id 3)
    (`KismetSystemLibrary.PrintString` (`KismetStringLibrary.Concat_StrStr` "PLAYED KILLED ENEMY: " (`KismetStringLibrary.Conv_IntToString` id)) true true (struct :`R` 1.0 :`G` 0.978046 :`A` 1.0))
    (else
      (`KismetSystemLibrary.PrintString` "IGNORE ENEMY NOTIFY" true true (struct :`R` 1.0 :`G` 0.041897 :`A` 1.0)))))

(fn `UserConstructionScript`)